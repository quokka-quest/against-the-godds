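; BP_GameManager builds the game's room map through GenerateMap, returning a shuffled list of room types.
; It splits TotalRooms into a fifth rest rooms, with the remainder halved between combat and non-combat rooms.
; Each shuffled room becomes a MapNodes entry, with the first marked visited and set as the current node.
; Generation runs only while AllRooms is empty; later calls return the existing list.
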(fn `GenerateMap`
  (returns (MapLayout :type "Array of /Game/System_OWMap/EMapRoomType Enum"))
  (bind _output_roomtype (break `/Game/ST_MapNodeData` (`|GetArrayItem` (`self.MapNodes`))))
  (if (`KismetArrayLibrary.Array_IsEmpty` (`self.AllRooms`))
    (set `self.RestCount` (/ (`self.TotalRooms`) 5))
    (set `self.CombatCount` (/ (- (`self.TotalRooms`) (`self.RestCount`)) 2))
    (set `self.NonCombatCount` (/ (- (`self.TotalRooms`) (`self.RestCount`)) 2))
    (for _ (range 1 (+ (`self.RestCount`) 1))
      (`KismetArrayLibrary.Array_Add` (`self.AllRooms`) "NewEnumerator2"))
    (for _ (range 1 (+ (`self.CombatCount`) 1))
      (`KismetArrayLibrary.Array_Add` (`self.AllRooms`) "NewEnumerator0"))
    (for _ (range 1 (+ (`self.NonCombatCount`) 1))
      (`KismetArrayLibrary.Array_Add` (`self.AllRooms`) "NewEnumerator1"))
    (`KismetArrayLibrary.Array_Shuffle` (`self.AllRooms`))
    (for _array_element (`self.AllRooms`)
      (bind _output_get (set `self.MapDataStruct` (make `/Game/ST_MapNodeData` _array_element)))
      (`KismetArrayLibrary.Array_Add` (`self.MapNodes`) _output_get))
    (`KismetArrayLibrary.Array_Set` (`self.MapNodes`) 0 (make `/Game/ST_MapNodeData` _output_roomtype true))
    (set `self.CurrentNodeIndex` 0)
    (return (`self.AllRooms`))
    (else
      (return (`self.AllRooms`)))))