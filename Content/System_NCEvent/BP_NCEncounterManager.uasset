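; BP_NCEncounterManager selects a noncombat encounter and shows it on screen when play begins.
; It reads every DT_Encounters row, keeping those that are repeatable or not yet completed according to the GameManager game instance.
; The last available entry becomes CurrentEncounter and feeds a new WBP_NoncombatEncounter widget added to the viewport.
; A random-index node is present but unused, and the list is not checked for being empty.
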(event `self.ReceiveBeginPlay`
  (bind _availableencounters (`self.AvailableEncounters`))
  (bind _asgame_manager (cast `GameManager` (`GameplayStatics.GetGameInstance`)))
  (set `self.GameManager` _asgame_manager)
  (bind _outrownames (`DataTableFunctionLibrary.GetDataTableRowNames` "/Game/System_NCEvent/DT_Encounters.DT_Encounters"))
  (for _array_element _outrownames
    (bind _returnvalue (`|GetDataTableRow` "/Game/System_NCEvent/DT_Encounters.DT_Encounters" _array_element)
      (:`then`
        (bind _output_get (set `self.Encounter` _returnvalue))
        (bind _returnvalue_2 (`GameManager.isEncounterCompleted` (`self.GameManager`) (break `/Game/System_NCEvent/ST_EncounterData` _output_get)))
        (if (or (== _returnvalue_2 false) (`.IsRepeatable_16_37B9428E41048356178D1CB6A56F2DDE` (break `/Game/System_NCEvent/ST_EncounterData` _output_get)))
          (`KismetArrayLibrary.Array_AddUnique` (`self.AvailableEncounters`) (`self.Encounter`))))))
  (bind _output_get_2 (set `self.CurrentEncounter` (`|GetArrayItem` _availableencounters (`KismetArrayLibrary.Array_LastIndex` _availableencounters))))
  (bind _returnvalue_3 (`|CreateWidget` "/Game/System_NCEvent/WBP_NoncombatEncounter.WBP_NoncombatEncounter_C" null _output_get_2))
  (`UserWidget.AddToViewport` _returnvalue_3 0))

(fn `UserConstructionScript`)