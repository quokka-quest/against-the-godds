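; BP_MapManager tracks the current node on a room map and holds disconnected logic for building that map's UI.
; Its functions check whether a clicked node connects to the current one, and set a new current node with its marker shown.
; BeginPlay and Tick are empty, so the graph that generates GameManager map nodes, chains WBP_MapNodeButton widgets in WBP_Map and appends rest and boss nodes never runs, nor does older room-shuffle scaffolding.
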(event `self.ReceiveTick`
  (params (DeltaSeconds :type "Float (single-precision)")))

(event `self.ReceiveBeginPlay`)

(fn `CheckIfConnectedNode`
  (params (ClickedNode :type "/Game/System_OWMap/WBP_MapNodeButton Object Reference"))
  (returns (`IsConnected?` :type Boolean))
  (bind _returnvalue (`KismetArrayLibrary.Array_Contains` (`/Game/System_OWMap/WBP_MapNodeButton.ConnectedNodes` (`self.CurrentNode`)) ClickedNode))
  (if _returnvalue
    (return _returnvalue)
    (else
      (return _returnvalue))))

(fn `SetNewCurrentNode`
  (params (NewCurrentNode :type "/Game/System_OWMap/WBP_MapNodeButton Object Reference"))
  (bind _output_get (set `self.CurrentNode` NewCurrentNode))
  (`Widget.SetVisibility` (`/Game/System_OWMap/WBP_MapNodeButton.TextBlock_0` _output_get) "Visible")
  (return))

(fn `UserConstructionScript`)