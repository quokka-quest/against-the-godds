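; BP_HomeScreenCam is a camera pawn that sets up the home screen when play begins.
; PossessThis makes it the first player controller's view target and possessed pawn, shows the mouse cursor, and destroys a DefaultPawn actor if one exists.
; BeginPlay then creates the WB_HomeScreen widget and adds it to the viewport.
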(event `self.ReceiveBeginPlay`
  (`self.PossessThis`)
  (bind _returnvalue (`|CreateWidget` "/Game/UI/WB_HomeScreen.WB_HomeScreen_C"))
  (`UserWidget.AddToViewport` _returnvalue 0))

(fn `PossessThis`
  (bind _returnvalue (`GameplayStatics.GetPlayerController` 0))
  (`PlayerController.SetViewTargetWithBlend` _returnvalue self 0.0 "VTBlend_Linear" 0.0 false)
  (`Controller.Possess` _returnvalue self)
  (set `PlayerController.bShowMouseCursor` true (`GameplayStatics.GetPlayerController` 0))
  (bind _returnvalue_2 (`GameplayStatics.GetActorOfClass` "/Script/Engine.DefaultPawn"))
  (if (`KismetSystemLibrary.IsValid` _returnvalue_2)
    (`self.K2_DestroyActor` _returnvalue_2)))

(fn `UserConstructionScript`)