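; BP_TurnIndicator is a marker mesh that hovers above the combatant whose turn it is in combat.
; BeginPlay stores the BP_CombatGameMode as its combat manager and hides the mesh.
; Each Tick polls that manager for the current combatant and, if valid, shows the mesh at a fixed height above it, spinning it in yaw at a frame-rate-independent speed.
; The mesh is never hidden again after it first appears.
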(event `self.ReceiveBeginPlay`
  (bind _asbp_combat_game_mode (cast `/Game/Blueprints/GameModes/BP_CombatGameMode` (`GameplayStatics.GetGameMode`)))
  (set `self.CombatManager` _asbp_combat_game_mode)
  (`SceneComponent.SetVisibility` (`self.IndicatorMesh`) false false))

(event `self.ReceiveTick`
  (params (DeltaSeconds :type "Float (single-precision)"))
  (bind _combatmanager (`self.CombatManager`))
  (bind _returnvalue (`CombatManager.GetCurrentCombatant` _combatmanager))
  (bind _returnvalue_location (`KismetMathLibrary.BreakTransform` (`self.GetTransform` _returnvalue)))
  (`/Engine/EditorBlueprintResources/StandardMacros.IsValid` _combatmanager
    (:`Is Valid`
      (`/Engine/EditorBlueprintResources/StandardMacros.IsValid` _returnvalue
        (:`Is Valid`
          (`SceneComponent.K2_SetWorldLocation` (`self.IndicatorMesh`) (+ _returnvalue_location (0.0 0.0 250.0)) false false)
          (`SceneComponent.SetVisibility` (`self.IndicatorMesh`) true false)
          (`SceneComponent.K2_AddWorldRotation` (`self.IndicatorMesh`) (`KismetMathLibrary.MakeRotator` 0.0 0.0 (* DeltaSeconds 100.0)) false false))))))

(fn `UserConstructionScript`)