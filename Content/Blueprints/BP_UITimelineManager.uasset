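; UI animation manager that plays queued width shrink and grow animations on UMG images, sequenced through the arena's turn event queue.
; Enqueue events wrap the image in an instanced-struct payload and add the shrink or grow event to the queue taken from BP_Arena.
; Each handler uses a timeline to rebuild the brush, lerping width to zero or from zero to a fixed size, then marks the event complete.
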(event `self.ReceiveBeginPlay`
  (bind _returnvalue (`GameplayStatics.GetActorOfClass` "/Game/Blueprints/BP_Arena.BP_Arena_C"))
  (set `self.QueueName` (`/Game/Blueprints/BP_Arena.TurnEventQueue` _returnvalue)))

(event `EnqueueImageShrink`
  (params (Image :type "Image Object Reference"))
  (bind _returnvalue (`BlueprintInstancedStructLibrary.MakeInstancedStruct` (make `/Game/EnumsAndStructs/S_ImagePayload` Image)))
  (`EventQueueBlueprintHandler.EnqueueEvent` (delegate `ShrinkImage`) _returnvalue (`self.QueueName`) "None" 0 1))

(event `ShrinkImage`
  (params (Payload :type "InstancedStruct Structure"))
  (bind _initialshrinkbrush (`self.InitialShrinkBrush`))
  (bind _value (`BlueprintInstancedStructLibrary.GetInstancedStructValue` Payload)
    (:`Valid`
      (bind _output_get (set `self.TargetImage` (`.Image_2_D2D35D4540798CA213979B9AA1020288` (break `/Game/EnumsAndStructs/S_ImagePayload` _value))))
      (set `self.InitialShrinkBrush` (`Image.Brush` _output_get))
      (bind (_direction _newtrack_0) (`Timeline|UITimeline` :!via `PlayFromStart`)
        (:`Update`
          (`Image.SetBrush` (`self.TargetImage`) (make `SlateBrush` (break `SlateBrush` _initialshrinkbrush) (`.DrawAs` (break `SlateBrush` _initialshrinkbrush)) (`.Tiling` (break `SlateBrush` _initialshrinkbrush)) (`.Mirroring` (break `SlateBrush` _initialshrinkbrush)) (make `DeprecateSlateVector2D` (`KismetMathLibrary.Lerp` (break `DeprecateSlateVector2D` (`.ImageSize` (break `SlateBrush` _initialshrinkbrush))) 0.0 _newtrack_0) (`.Y` (break `DeprecateSlateVector2D` (`.ImageSize` (break `SlateBrush` _initialshrinkbrush))))) (`.Margin` (break `SlateBrush` _initialshrinkbrush)) (`.ResourceObject` (break `SlateBrush` _initialshrinkbrush)) (`.OutlineSettings` (break `SlateBrush` _initialshrinkbrush)))))
        (:`Finished`
          (`EventQueueSystem.MarkEventAsComplete` (subsystem `EventQueueSystem`) (`self.QueueName`)))))))

(event `EnqueueImageGrowth`
  (params (Image :type "Image Object Reference"))
  (bind _returnvalue (`BlueprintInstancedStructLibrary.MakeInstancedStruct` (make `/Game/EnumsAndStructs/S_ImagePayload` Image)))
  (`EventQueueBlueprintHandler.EnqueueEvent` (delegate `GrowImage`) _returnvalue (`self.QueueName`) "None" 0 1))

(event `GrowImage`
  (params (Payload :type "InstancedStruct Structure"))
  (bind _initialgrowbrush (`self.InitialGrowBrush`))
  (bind _value (`BlueprintInstancedStructLibrary.GetInstancedStructValue` Payload)
    (:`Valid`
      (bind _output_get (set `self.TargetImage` (`.Image_2_D2D35D4540798CA213979B9AA1020288` (break `/Game/EnumsAndStructs/S_ImagePayload` _value))))
      (set `self.InitialGrowBrush` (`Image.Brush` _output_get))
      (bind (_direction _floattrack) (`Timeline|Timeline` :!via `PlayFromStart`)
        (:`Update`
          (`Image.SetBrush` (`self.TargetImage`) (make `SlateBrush` (break `SlateBrush` _initialgrowbrush) (`.DrawAs` (break `SlateBrush` _initialgrowbrush)) (`.Tiling` (break `SlateBrush` _initialgrowbrush)) (`.Mirroring` (break `SlateBrush` _initialgrowbrush)) (make `DeprecateSlateVector2D` (`KismetMathLibrary.Lerp` 0.0 64.0 _floattrack) (`.Y` (break `DeprecateSlateVector2D` (`.ImageSize` (break `SlateBrush` _initialgrowbrush))))) (`.Margin` (break `SlateBrush` _initialgrowbrush)) (`.ResourceObject` (break `SlateBrush` _initialgrowbrush)) (`.OutlineSettings` (break `SlateBrush` _initialgrowbrush)))))
        (:`Finished`
          (`EventQueueSystem.MarkEventAsComplete` (subsystem `EventQueueSystem`) (`self.QueueName`)))))))

(fn `UserConstructionScript`)