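; Base actor for turn-based arena combatants, handling tile movement, per-turn movement points, simple fixed-damage attacks and a camera-facing health bar.
; MoveToTile checks BP_Arena's walkable tiles, spends movement, then lerps players immediately via timeline.
; Non-players instead queue moves on the event queue system with instanced-struct payloads, marking each complete so they run sequentially.
; Both movement paths refresh arena tile colours, occupancy and walkability on arrival.
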(event `self.ReceiveBeginPlay`
  (bind _returnvalue (`GameplayStatics.GetActorOfClass` "/Game/Blueprints/BP_Arena.BP_Arena_C"))
  (set `self.ArenaRef` _returnvalue)
  (set `self.CurrentHealth` (`self.MaxHealth`))
  (bind _aswb_healthbar (cast `/Game/UI/WB_Healthbar` (`WidgetComponent.GetWidget` (`self.HealthWidget`))))
  (`/Game/UI/WB_Healthbar.Initialise` _aswb_healthbar self))

(event `self.ReceiveTick`
  (params (DeltaSeconds :type "Float (single-precision)"))
  (`self.UpdateHealthBarRotation`))

(event `MoveToTargetTile`
  (params (CurrentPos :type "Vector Structure") (TargetPos :type "Vector Structure"))
  (bind _arenaref (`self.ArenaRef`))
  (bind (_direction _newtrack_0) (`Timeline|MoveTime` :!via `PlayFromStart`)
    (:`Update`
      (`SceneComponent.K2_SetWorldLocation` (`self.DefaultSceneRoot`) (`KismetMathLibrary.VLerp` CurrentPos TargetPos _newtrack_0) false false))
    (:`Finished`
      (`SceneComponent.K2_SetWorldLocation` (`self.DefaultSceneRoot`) TargetPos false false)
      (`/Game/Blueprints/BP_Arena.ResetAllTileColour` _arenaref)
      (`/Game/Blueprints/BP_Arena.UpdateOccupiedTiles` _arenaref)
      (`/Game/Blueprints/BP_Arena.UpdateWalkableTiles` _arenaref))))

(event `EnqueueMovement`
  (params (CurrentPos :type "Vector Structure") (TargetPos :type "Vector Structure"))
  (bind _returnvalue (`BlueprintInstancedStructLibrary.MakeInstancedStruct` (make `/Game/EnumsAndStructs/S_MoveVectors` CurrentPos TargetPos)))
  (`EventQueueBlueprintHandler.EnqueueEvent` (delegate `AIMoveEvent`) _returnvalue "UIQueue" "None" 0 1))

(event `AIMoveEvent`
  (params (Payload :type "InstancedStruct Structure"))
  (bind _arenaref (`self.ArenaRef`))
  (bind _value (`BlueprintInstancedStructLibrary.GetInstancedStructValue` Payload)
    (:`Valid`
      (bind (_direction _newtrack_0) (`Timeline|Timeline` :!via `PlayFromStart`)
        (:`Update`
          (bind (_startpos _targetpos) (break `/Game/EnumsAndStructs/S_MoveVectors` _value))
          (`SceneComponent.K2_SetWorldLocation` (`self.DefaultSceneRoot`) (`KismetMathLibrary.VLerp` _startpos _targetpos _newtrack_0) false false))
        (:`Finished`
          (`SceneComponent.K2_SetWorldLocation` (`self.DefaultSceneRoot`) _targetpos false false)
          (`/Game/Blueprints/BP_Arena.ResetAllTileColour` _arenaref)
          (`/Game/Blueprints/BP_Arena.UpdateOccupiedTiles` _arenaref)
          (`/Game/Blueprints/BP_Arena.UpdateWalkableTiles` _arenaref)
          (`EventQueueSystem.MarkEventAsComplete` (subsystem `EventQueueSystem`) "UIQueue"))))))

(fn `AttackTarget`
  (params (Target :type "/Game/Blueprints/BP_Entity Object Reference"))
  (set `/Game/Blueprints/BP_Entity.CurrentHealth` (`KismetMathLibrary.FClamp` (- (`/Game/Blueprints/BP_Entity.CurrentHealth` Target) 2.0) 0.0 (`/Game/Blueprints/BP_Entity.MaxHealth` Target)) Target))

(fn `FinishTurn`)

(fn `InitialiseTurn`
  (`/Game/Blueprints/BP_Arena.ChangeTilesColour` (`self.ArenaRef`) (`self.CurrentTile`) "/Game/Materials/M_TileGold.M_TileGold")
  (set `self.availableMovement` (`self.TotalMovement`)))

(fn `IsTargetTileValid`
  (params (TileIndex :type Integer))
  (returns (IsValid :type Boolean))
  (bind _arenaref (`self.ArenaRef`))
  (bind (_x _y) (`/Game/Blueprints/BP_Arena.GetTileCoordsFromIndex` _arenaref TileIndex))
  (bind (_x_2 _y_2) (`/Game/Blueprints/BP_Arena.GetTileCoordsFromIndex` _arenaref (`self.CurrentTile`)))
  (return (and (<= (`KismetMathLibrary.Abs_Int` (- _x_2 _x)) 1) (<= (`KismetMathLibrary.Abs_Int` (- _y_2 _y)) 1))))

(fn `MoveToTile`
  (params (NewTileNum :type Integer))
  (locals (Tile :type "/Game/Blueprints/BP_Tile Object Reference"))
  (bind _arenaref (`self.ArenaRef`))
  (bind _returnvalue (`SceneComponent.K2_GetComponentLocation` (`self.DefaultSceneRoot`)))
  (bind _returnvalue_2 (`SceneComponent.K2_GetComponentLocation` (`|GetArrayItem` (`/Game/Blueprints/BP_Arena.GridArray` _arenaref) NewTileNum)))
  (if (> (`self.availableMovement`) 0)
    (if (`KismetArrayLibrary.Array_Contains` (`/Game/Blueprints/BP_Arena.CurrentWalkableTileIndices` _arenaref) NewTileNum)
      (set `self.CurrentTile` (`local.NewTileNum`))
      (`/Engine/EditorBlueprintResources/StandardMacros.DecrementInt` (`self.availableMovement`)
        (:`  `
          (cast `/Game/Blueprints/BP_Player` self
            (:`then`
              (`self.MoveToTargetTile` _returnvalue _returnvalue_2))
            (:`CastFailed`
              (`self.EnqueueMovement` _returnvalue _returnvalue_2)))))
      (else
        (`KismetSystemLibrary.PrintString` "Tile Can't be moved to")))))

(fn `UpdateHealthBarRotation`
  (`SceneComponent.K2_SetWorldRotation` (`self.HealthWidget`) (`KismetMathLibrary.FindLookAtRotation` (`SceneComponent.K2_GetComponentLocation` (`self.HealthWidget`)) (`PlayerCameraManager.GetCameraLocation` (`GameplayStatics.GetPlayerCameraManager` 0))) false false))

(fn `UserConstructionScript`)