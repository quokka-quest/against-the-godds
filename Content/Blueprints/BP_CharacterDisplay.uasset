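; Character display actor that shows the chosen mesh for up to three players, likely for a character selection or lobby view.
; SetCharMesh switches on the player number, assigns the new static mesh to the matching P1, P2 or P3 component and makes it visible.
; HideCharMesh hides that player's component; the actor has no event or construction logic, so other Blueprints drive it through these functions.
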(fn `HideCharMesh`
  (params (PlayerNum :type "/Game/EnumsAndStructs/E_PlayerNums Enum" :default "NewEnumerator0"))
  (switch `/Game/EnumsAndStructs/E_PlayerNums` PlayerNum
    (:`NewEnumerator0`
      (`SceneComponent.SetVisibility` (`self.P1`) false false))
    (:`NewEnumerator1`
      (`SceneComponent.SetVisibility` (`self.P2`) false false))
    (:`NewEnumerator2`
      (`SceneComponent.SetVisibility` (`self.P3`) false false))))

(fn `SetCharMesh`
  (params (CharNum :type "/Game/EnumsAndStructs/E_PlayerNums Enum" :default "NewEnumerator0") (NewMesh :type "StaticMesh Object Reference"))
  (switch `/Game/EnumsAndStructs/E_PlayerNums` CharNum
    (:`NewEnumerator0`
      (`StaticMeshComponent.SetStaticMesh` (`self.P1`) (`local.NewMesh`))
      (`SceneComponent.SetVisibility` (`self.P1`) true false))
    (:`NewEnumerator1`
      (`StaticMeshComponent.SetStaticMesh` (`self.P2`) (`local.NewMesh`))
      (`SceneComponent.SetVisibility` (`self.P2`) true false))
    (:`NewEnumerator2`
      (`StaticMeshComponent.SetStaticMesh` (`self.P3`) (`local.NewMesh`))
      (`SceneComponent.SetVisibility` (`self.P3`) true false))))

(fn `UserConstructionScript`)