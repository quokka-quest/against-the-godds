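; BP_VFXManager is a manager actor that spawns short-lived visual effect actors on request, selected by an effect tag.
; TriggerSwirly spawns a BP_SwirlyPlayer at each target's XY location, and TriggerSingleUseVFX spawns a BP_SingleUseEffect at a single entity's XY location.
; TriggerChainEffect spawns a BP_ChainEffect and passes it start and end points.
; Each spawned actor receives the tag and handles playback itself.
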(event `TriggerSwirly`
  (params (Targets :type "Array of Actor Object Reference") (EffectTag :type "GameplayTag Structure"))
  (for _array_element Targets
    (bind (_returnvalue_x _returnvalue_y) (`KismetMathLibrary.BreakVector` (`self.K2_GetActorLocation` _array_element)))
    (bind _returnvalue (`|SpawnActorFromClass` "/Game/Blueprints/VFXRelated/BP_SwirlyPlayer.BP_SwirlyPlayer_C" (`KismetMathLibrary.MakeTransform` (`KismetMathLibrary.MakeVector` _returnvalue_x _returnvalue_y)) "Undefined" "MultiplyWithRoot" null null))
    (`/Game/Blueprints/VFXRelated/BP_SwirlyPlayer.PlaySwirly` _returnvalue EffectTag)))

(event `TriggerSingleUseVFX`
  (params (TargetEntity :type "Actor Object Reference") (EffectTag :type "GameplayTag Structure"))
  (bind (_returnvalue_x _returnvalue_y) (`KismetMathLibrary.BreakVector` (`self.K2_GetActorLocation` TargetEntity)))
  (bind _returnvalue (`|SpawnActorFromClass` "/Game/Blueprints/VFXRelated/BP_SingleUseEffect.BP_SingleUseEffect_C" (`KismetMathLibrary.MakeTransform` (`KismetMathLibrary.MakeVector` _returnvalue_x _returnvalue_y)) "Undefined" "MultiplyWithRoot" null null))
  (`/Game/Blueprints/VFXRelated/BP_SingleUseEffect.TriggerEffect` _returnvalue EffectTag))

(event `TriggerChainEffect`
  (params (Tag :type "GameplayTag Structure") (StartPos :type "Vector Structure") (EndPos :type "Vector Structure"))
  (bind _returnvalue (`|SpawnActorFromClass` "/Game/Blueprints/VFXRelated/BP_ChainEffect.BP_ChainEffect_C" (`KismetMathLibrary.MakeTransform` (0.0 0.0 0.0)) "Undefined" "MultiplyWithRoot" null null))
  (`/Game/Blueprints/VFXRelated/BP_ChainEffect.SetChainPoints` _returnvalue Tag StartPos EndPos))

(fn `UserConstructionScript`)