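; BP_SwirlyPlayer is a short-lived VFX actor that plays a Niagara "swirly" effect chosen by tag.
; PlaySwirly looks the tag up in SwirlyTagMap, then assigns and activates that system, or destroys the actor when no match exists.
; While playing, it raises BP_ActivityManager's active animation count, lowers it after a fixed delay, then destroys itself after a second delay.
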(event `self.ReceiveBeginPlay`
  (bind _returnvalue (`GameplayStatics.GetActorOfClass` "/Game/Blueprints/Managers/BP_ActivityManager.BP_ActivityManager_C"))
  (set `self.ActivityRef` _returnvalue))

(event `MarkActivityOngoing`
  (`/Game/Blueprints/Managers/BP_ActivityManager.IncrementActiveAnims` (`self.ActivityRef`))
  (`KismetSystemLibrary.Delay` 3.0)
  (`/Game/Blueprints/Managers/BP_ActivityManager.DecrementActiveAnims` (`self.ActivityRef`))
  (`KismetSystemLibrary.Delay` 3.0)
  (`self.K2_DestroyActor`))

(event `PlaySwirly`
  (params (EffectTag :type "GameplayTag Structure"))
  (bind (_value _returnvalue) (`BlueprintMapLibrary.Map_Find` (`self.SwirlyTagMap`) EffectTag))
  (if _returnvalue
    (`self.MarkActivityOngoing`)
    (`NiagaraComponent.SetAsset` (`self.Niagara`) _value true)
    (`ActorComponent.Activate` (`self.Niagara`) false)
    (else
      (`self.K2_DestroyActor`))))

(fn `UserConstructionScript`)