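; BP_SingleUseEffect is a short-lived effect actor that plays a Niagara effect chosen by tag.
; TriggerEffect looks up the tag in EffectVFXMap, then assigns and activates the matching system on its Niagara component.
; On BeginPlay it finds BP_ActivityManager and counts itself as an active animation for a fixed delay.
; After releasing that count, it waits again and destroys itself, independent of whether an effect was triggered.
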(event `self.ReceiveBeginPlay`
  (bind _returnvalue (`GameplayStatics.GetActorOfClass` "/Game/Blueprints/Managers/BP_ActivityManager.BP_ActivityManager_C"))
  (set `self.Activity Ref` _returnvalue)
  (`self.MarkActivityOngoing`))

(event `MarkActivityOngoing`
  (`/Game/Blueprints/Managers/BP_ActivityManager.IncrementActiveAnims` (`self.Activity Ref`))
  (`KismetSystemLibrary.Delay` 3.0)
  (`/Game/Blueprints/Managers/BP_ActivityManager.DecrementActiveAnims` (`self.Activity Ref`))
  (`KismetSystemLibrary.Delay` 3.0)
  (`self.K2_DestroyActor`))

(event `TriggerEffect`
  (params (EffectTag :type "GameplayTag Structure"))
  (bind (_value _returnvalue) (`BlueprintMapLibrary.Map_Find` (`self.EffectVFXMap`) EffectTag))
  (if _returnvalue
    (`NiagaraComponent.SetAsset` (`self.Niagara`) _value true)
    (`ActorComponent.Activate` (`self.Niagara`) false)))

(fn `UserConstructionScript`)