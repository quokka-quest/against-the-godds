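; Short-lived VFX actor that draws a Niagara beam between two points for tagged chain effects such as heal links, then destroys itself after two seconds.
; SetChainPoints looks up the Niagara system for the effect tag in TagMap and swaps it onto the component.
; It sets beam endpoints at a fixed height, ignoring input Z, and uses lighter spawn and spiral counts for HealLink before activating.
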(event `self.ReceiveBeginPlay`
  (`KismetSystemLibrary.Delay` 2.0)
  (`self.K2_DestroyActor`))

(event `SetChainPoints`
  (params (EffectTag :type "GameplayTag Structure") (Start :type "Vector Structure") (End :type "Vector Structure"))
  (bind _returnvalue (== EffectTag (struct :`TagName` "Buff.HealLink")))
  (bind (_value _returnvalue_2) (`BlueprintMapLibrary.Map_Find` (`self.TagMap`) EffectTag))
  (if _returnvalue_2
    (`NiagaraComponent.SetAsset` (`self.Niagara`) _value true)
    (`NiagaraComponent.SetVariableVec3` (`self.Niagara`) "Beam Start" (`KismetMathLibrary.MakeVector` (.x Start) (.y Start) 100.0))
    (`NiagaraComponent.SetVariableVec3` (`self.Niagara`) "Beam End" (`KismetMathLibrary.MakeVector` (.x End) (.y End) 100.0))
    (`NiagaraComponent.SetVariableInt` (`self.Niagara`) "Plus Spawn" (select `bool` _returnvalue :`false` 7 :`true` 5))
    (`NiagaraComponent.SetVariableInt` (`self.Niagara`) "Spiral Amount" (select `bool` _returnvalue :`false` 20 :`true` 15))
    (`ActorComponent.Activate` (`self.Niagara`) false)))

(fn `UserConstructionScript`)