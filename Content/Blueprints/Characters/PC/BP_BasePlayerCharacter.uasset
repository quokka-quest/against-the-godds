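; BP_BasePlayerCharacter is a player character Blueprint that implements experience and talent point progression.
; AddXP adds to a cumulative XP pool and, on reaching the threshold, grants one talent point and multiplies the next threshold.
; The threshold is checked once per call, so a large gain yields only one level.
; A debug function wraps AddXP, and the event graph holds only disabled default events.
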(fn `AddXP`
  (params (XPToAdd :type Integer))
  ; Add the xp to the xp pool
  (set `self.XP` (+ XPToAdd (`self.XP`)))
  ; Enough to level up?
  (if (>= (`self.XP`) (`self.XPToNextLevel`))
    ;[0.15 1 0.15 0.5] Increase talent points
    (`/Engine/EditorBlueprintResources/StandardMacros.IncrementInt` (`self.TalentPoints`)
      (:`  `
        ; Increase the xp needed for the next level
        (set `self.XPToNextLevel` (* (`self.XPToNextLevel`) (`self.XPToNextLevelMultiplier`)))))))

(fn `AddXP DEBUG`
  (`self.AddXP` (`self.XPToAdd`)))

(fn `UserConstructionScript`
  (`parent.UserConstructionScript`))