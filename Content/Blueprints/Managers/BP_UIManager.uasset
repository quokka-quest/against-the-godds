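; UI manager for turn-based combat that relays requests to the player turn and turn order widgets.
; It toggles the dice cam and ability buttons, refreshes an entity's abilities, removes entities from the turn order and clears the highlighted entity.
; It caches the combat game mode on BeginPlay, so the delayed dice cam shutdown re-enables ability buttons only when the current combatant is a player entity.
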(event `self.ReceiveBeginPlay`
  (bind _asbp_combat_game_mode (cast `/Game/Blueprints/GameModes/BP_CombatGameMode` (`GameplayStatics.GetGameMode`)))
  (set `self.CombatManagerRef` _asbp_combat_game_mode))

(event `DisableDiceCamWithDelay`
  (params (Delay :type "Float (double-precision)"))
  (`KismetSystemLibrary.Delay` Delay)
  (`/Game/UI/Combat/WB_PlayerTurnUI.ToggleDiceCam` (`self.PlayerTurnUI`) false)
  (cast `PlayerEntity` (`CombatManager.CurrentTurnCombatant` (`self.CombatManagerRef`)))
  (`/Game/UI/Combat/WB_PlayerTurnUI.ToggleAbilityButtons` (`self.PlayerTurnUI`) true))

(fn `RemoveEntityFromTurnOrder`
  (params (Entity :type "EntityBase Object Reference"))
  (`/Game/UI/Combat/WB_CombatUI.RemoveCombatantOnDeath` (`self.TurnOrderUI`) Entity))

(fn `RemoveEntityHighlight`
  (set `self.EntityToHighlight` null))

(fn `ToggleAbilityButtons`
  (params (Enable :type Boolean))
  (`/Game/UI/Combat/WB_PlayerTurnUI.ToggleAbilityButtons` (`self.PlayerTurnUI`) Enable))

(fn `ToggleDiceCam`
  (params (Enable :type Boolean))
  (`/Game/UI/Combat/WB_PlayerTurnUI.ToggleDiceCam` (`self.PlayerTurnUI`) Enable))

(fn `UpdateAbilityButtons`
  (params (entity :type "EntityBase Object Reference"))
  (`/Game/UI/Combat/SubWidgets/WBP_AttackMenu.UpdateAbilities` (`/Game/UI/Combat/WB_PlayerTurnUI.WBP_AttackMenu` (`self.PlayerTurnUI`)) entity))

(fn `UserConstructionScript`)