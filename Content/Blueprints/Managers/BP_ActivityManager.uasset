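; Manager actor that tracks active animations during turn-based combat so UI and enemy turns wait for them to finish.
; A counter rises and falls as animations start and end, disabling player buttons while any are active.
; At zero, it ends the turn of a single marked enemy after a two-tick delay.
; It re-enables player buttons if the combat game mode's current combatant is a player.
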(event `self.ReceiveBeginPlay`
  (`self.SetReferenceVars`))

(event `OnAllAnimsFinished`
  (`KismetSystemLibrary.PrintString` "Every Animation marked as finished" true false (struct :`R` 1.0 :`G` 0.025834 :`A` 1.0) 5.0)
  (`|ExecutionSequence`
    (:`then_0`
      ;[1 0 0 0.5 30] If an enemy is marked for its turn to end, then end that enemies turn
      (`/Engine/EditorBlueprintResources/StandardMacros.IsValid` (`self.EnemyRef`)
        (:`Is Valid`
          (`KismetSystemLibrary.DelayUntilNextTick`)
          (`KismetSystemLibrary.DelayUntilNextTick`)
          (`EntityBase.OnTurnEnd` (`self.EnemyRef`))
          (set `self.EnemyRef` null))))
    (:`then_1`
      ;[1 0 0 0.5 30] If it is a player's turn, enable the UI when animations have completed
      (cast `PlayerEntity` (`CombatManager.GetCurrentCombatant` (`self.CombatManagerRef`)))
      (`/Game/Blueprints/Managers/BP_UIManager.ToggleAllPlayerButtons` (`self.UiManagerRef`) true))))

(fn `DecrementActiveAnims`
  (bind _output_get (set `self.ActiveAnims` (`KismetMathLibrary.Max` (- (`self.ActiveAnims`) 1))))
  (if (== _output_get 0)
    (`self.OnAllAnimsFinished`)))

(fn `IncrementActiveAnims`
  (`/Engine/EditorBlueprintResources/StandardMacros.IncrementInt` (`self.ActiveAnims`)
    (:`  `
      (`/Game/Blueprints/Managers/BP_UIManager.ToggleAllPlayerButtons` (`self.UiManagerRef`) false))))

(fn `MarkEnemyForTurnEndOnAnimsDone`
  (params (Entity :type "EnemyEntity Object Reference"))
  (`/Engine/EditorBlueprintResources/StandardMacros.IsValid` (`self.EnemyRef`)
    (:`Is Valid`
      (`KismetSystemLibrary.PrintString` "Error: BP_ActivityManager->MarkEnemyForTurnEndOnAnimsDone: Attempted to mark an enemy when an enemy was already marked" true true (struct :`G` 0.66 :`B` 1.0 :`A` 1.0) 20.0))
    (:`Is Not Valid`
      (set `self.EnemyRef` (`local.Entity`)))))

(fn `SetReferenceVars`
  (`|ExecutionSequence`
    (:`then_0`
      (bind _returnvalue (`GameplayStatics.GetActorOfClass` "/Game/Blueprints/Managers/BP_UIManager.BP_UIManager_C"))
      (set `self.UiManagerRef` _returnvalue))
    (:`then_1`
      (bind _asbp_combat_game_mode (cast `/Game/Blueprints/GameModes/BP_CombatGameMode` (`GameplayStatics.GetGameMode`)))
      (set `self.CombatManagerRef` _asbp_combat_game_mode))))

(fn `UserConstructionScript`)