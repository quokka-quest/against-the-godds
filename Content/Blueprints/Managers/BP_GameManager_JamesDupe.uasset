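; Game manager that holds run state (relics, character abilities, tutorial progress) and controls music that persists across level transitions.
; Relics are de-duplicated, with Game Mode types also stored as permanent effects, and cleared on reset.
; Tutorials, gated by a save setting, pick a data table by level name to feed a message widget.
; Ability drafts draw unowned abilities from per-character data tables, seeding one damage pick plus two random others.
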(event `self.ReceiveInit`)

(event `PlaySound`
  (params (SoundToPlay :type "SoundWave Object Reference"))
  (`/Engine/EditorBlueprintResources/StandardMacros.IsValid` (`self.AudioComponentRef`)
    (:`Is Valid`
      (if (not (== SoundToPlay (`self.CurrentMusic`)))
        (`AudioComponent.Stop` (`self.AudioComponentRef`))
        (bind _returnvalue (`GameplayStatics.SpawnSound2D` SoundToPlay 1.0 1.0 0.0 null true :!label _label))
        (set `self.AudioComponentRef` _returnvalue)
        (set `self.CurrentMusic` SoundToPlay)))
    (:`Is Not Valid`
      (goto _label))))

(event `StopMusic`
  (`AudioComponent.Stop` (`self.AudioComponentRef`)))

(fn `ActivateTutorial`
  (set `self.TutorialActive` true))

(fn `AddAbility`
  (params (ChosenAbility :type "GameplayAbility Class Reference") (Character :type "PlayerEntity Class Reference"))
  (bind (_keypin _valuepin) (`|MapForEach` (`self.CharacterInfo`))
    (:`then`
      (if (== _keypin Character)
        (`KismetArrayLibrary.Array_AddUnique` (break `PersistentPlayerInfo` _valuepin) ChosenAbility)))))

(fn `AddRelic`
  (params (RelicToAdd :type "/Game/System_NCEvent/RelicSystem/ST_RelicRow Structure"))
  (bind _currentrelics (`self.CurrentRelics`))
  (bind (_relic_to_add_name _relic_to_add_gameplayeffect _relic_to_add_onstackchange _relic_to_add_description _relic_to_add_icon _relic_to_add_applicationtype) (break `/Game/System_NCEvent/RelicSystem/ST_RelicRow` (`self.Relic to Add`)))
  (set `self.Relic to Add` RelicToAdd)
  (if (`KismetArrayLibrary.Array_Contains` _currentrelics (`self.Relic to Add`))
    (`KismetSystemLibrary.PrintString` "Already Obtained")
    (else
      (`KismetArrayLibrary.Array_AddUnique` _currentrelics (`self.Relic to Add`))
      (switch `/Game/System_NCEvent/RelicSystem/ENUM_RelicApplication` _relic_to_add_applicationtype
        (:`NewEnumerator2`
          (if (not (`KismetArrayLibrary.Array_Contains` (`self.PermanentRelicEffects`) (`self.Relic to Add`)))
            (`KismetArrayLibrary.Array_AddUnique` (`self.PermanentRelicEffects`) (`self.Relic to Add`))
            (for _array_element (`self.PermanentRelicEffects`)
              (`KismetSystemLibrary.PrintString` (break `/Game/System_NCEvent/RelicSystem/ST_RelicRow` _array_element)))))))))

(fn `CheckTutorialActive`
  (params (LevelName :type String))
  (returns (TutorialActive :type Boolean))
  (bind _enabled (`/MenuUI/Blueprints/BP_SettingSaveSubsystem.GetTutorialSetting` (subsystem `/MenuUI/Blueprints/BP_SettingSaveSubsystem`)))
  (set `self.Level Name` LevelName)
  (if _enabled
    (`self.StartTutorialForLevel` (`self.Level Name`))
    (return _enabled)
    (else
      (return _enabled))))

(fn `CreateAbilityDraft`
  (bind _character_draft_abilities (`self.Character_Draft_Abilities`))
  (set `self.Counter` 0)
  ; Loops through character info to get each character that has been chosen
  (bind (_keypin _valuepin) (`|MapForEach` (`self.CharacterInfo`))
    (:`then`
      (`/Engine/EditorBlueprintResources/StandardMacros.IncrementInt` (`self.Counter`)
        (:`  `
          ; Clear a bunch of arrays that I need for each character in the loop
          (`KismetArrayLibrary.Array_Clear` (`self.DamageAbilityDraft`))
          (`KismetArrayLibrary.Array_Clear` (`self.AllAbilityDraft`))
          (`KismetArrayLibrary.Array_Clear` (`self.Character_Draft_Abilities`))
          (bind (_value _returnvalue) (`BlueprintMapLibrary.Map_Find` (`self.AbilityClassMap`) _keypin))
          (if _returnvalue
            ; Get each row from the data table
            (bind _outrownames (`DataTableFunctionLibrary.GetDataTableRowNames` _value))
            (for _array_element _outrownames
              (bind _returnvalue_2 (`|GetDataTableRow` _value _array_element)
                (:`then`
                  (bind (_abilityname _abilitytype _abilityref) (break `/Game/Data/ST_Ability` _returnvalue_2))
                  (if (not (`KismetArrayLibrary.Array_Contains` (break `PersistentPlayerInfo` _valuepin) _abilityref))
                    (bind _returnvalue_3 (`|GenericCreateObject` _abilityref))
                    ; Make arrays of all abilities and of specifically damage abilites to draft (we want a damage one seeded)
                    (`KismetArrayLibrary.Array_AddUnique` (`self.AllAbilityDraft`) _returnvalue_3)
                    (if (== _abilitytype 0)
                      (`KismetArrayLibrary.Array_AddUnique` (`self.DamageAbilityDraft`) _returnvalue_3))))))
            (`KismetSystemLibrary.PrintString` (`KismetStringLibrary.Concat_StrStr` "All Ability Draft length: " (`KismetStringLibrary.Conv_IntToString` (`KismetArrayLibrary.Array_Length` (`self.AllAbilityDraft`)))))
            (`KismetSystemLibrary.PrintString` (`KismetStringLibrary.Concat_StrStr` "Damage Ability Draft length: " (`KismetStringLibrary.Conv_IntToString` (`KismetArrayLibrary.Array_Length` (`self.DamageAbilityDraft`)))))
            (bind _output_get (set `self.DamageDrafted` (`KismetArrayLibrary.Array_Random` (`self.DamageAbilityDraft`))))
            (`KismetArrayLibrary.Array_Add` _character_draft_abilities _output_get)
            (bind _returnvalue_4 (`KismetArrayLibrary.Array_RemoveItem` (`self.AllAbilityDraft`) _output_get))
            (`KismetSystemLibrary.PrintString` (`KismetStringLibrary.Conv_BoolToString` _returnvalue_4))
            (`KismetSystemLibrary.PrintString` (`KismetStringLibrary.Concat_StrStr` "Character Draft Abilities Length: " (`KismetStringLibrary.Conv_IntToString` (`KismetArrayLibrary.Array_Length` _character_draft_abilities))))
            (`KismetSystemLibrary.PrintString` (`KismetStringLibrary.Concat_StrStr` "All Ability Draft length: " (`KismetStringLibrary.Conv_IntToString` (`KismetArrayLibrary.Array_Length` (`self.AllAbilityDraft`)))))
            (for _ (range 2)
              (bind _output_get_2 (set `self.DraftedAbility` (`KismetArrayLibrary.Array_Random` (`self.AllAbilityDraft`))))
              (`KismetArrayLibrary.Array_AddUnique` (`self.Character_Draft_Abilities`) _output_get_2)
              (`KismetSystemLibrary.PrintString` (`KismetStringLibrary.Concat_StrStr` "Character Draft Abilities Length: " (`KismetStringLibrary.Conv_IntToString` (`KismetArrayLibrary.Array_Length` (`self.Character_Draft_Abilities`)))))
              (bind _returnvalue_5 (`KismetArrayLibrary.Array_RemoveItem` (`self.AllAbilityDraft`) (`self.DraftedAbility`)))
              (`KismetSystemLibrary.PrintString` (`KismetStringLibrary.Conv_BoolToString` _returnvalue_5)))
            (switch `int` (`self.Counter`)
              (:`1`
                (bind _output_get_3 (set `self.Character1DraftedAbilities` (`self.Character_Draft_Abilities`)))
                (`KismetSystemLibrary.PrintString` (`KismetStringLibrary.Concat_StrStr` "Character 1 Draft Length: " (`KismetStringLibrary.Conv_IntToString` (`KismetArrayLibrary.Array_Length` _output_get_3)))))
              (:`2`
                (set `self.Character2DraftedAbilities` (`self.Character_Draft_Abilities`)))
              (:`3`
                (set `self.Character3DraftedAbilities` (`self.Character_Draft_Abilities`))))))))))

(fn `CreateTutorialMessage`
  (params (TutorialSequence :type "Array of Name"))
  (set `self.TutorialSequence` TutorialSequence)
  (bind _returnvalue (`|CreateWidget` "/Game/UI/WBP_TutorialMessage.WBP_TutorialMessage_C"))
  (`UserWidget.AddToViewport` _returnvalue 100))

(fn `DeactivateTutorial`
  (set `self.TutorialActive` false)
  (`self.EndTutorialMode`))

(fn `ProgressTutorial`
  (returns (TutorialActive :type Boolean))
  (bind _tutorialsequence (`self.TutorialSequence`))
  (if (> (`KismetArrayLibrary.Array_Length` _tutorialsequence) 1)
    (`KismetArrayLibrary.Array_Remove` _tutorialsequence)
    (`self.ProgressTutorialSequence`)
    (return true)
    (else
      (`KismetArrayLibrary.Array_Clear` _tutorialsequence)
      (`self.DeactivateTutorial`)
      (return false))))

(fn `ResetRelics`
  (`KismetArrayLibrary.Array_Clear` (`self.CurrentRelics`))
  (`KismetArrayLibrary.Array_Clear` (`self.PermanentRelicEffects`))
  (set `self.RoomNumber` 0)
  (`BlueprintMapLibrary.Map_Clear` (`self.CharacterInfo`))
  (set `/MenuUI/SaveGame/SG_UserSettings.GameplaySettings` (make `/MenuUI/Structs/S_GameplaySettings` false) (`/MenuUI/Blueprints/BP_SettingSaveSubsystem.SG_Settings` (subsystem `/MenuUI/Blueprints/BP_SettingSaveSubsystem`))))

(fn `StartTutorialForLevel`
  (params (LevelName :type String))
  ; IF YOU CHANGE TUTORIAL LEVEL, CHANGE PIN 2 STRING
  (`KismetArrayLibrary.Array_Clear` (`self.TutorialSequence`))
  (switch `string` LevelName
    (:`L_HomeScreenLevel`
      (bind _outrownames (`DataTableFunctionLibrary.GetDataTableRowNames` "/Game/Data/DT_Tutorials.DT_Tutorials"))
      (`self.CreateTutorialMessage` _outrownames))
    (:`L_MapScreen`
      (bind _outrownames_2 (`DataTableFunctionLibrary.GetDataTableRowNames` "/Game/Data/DT_MapTutorials.DT_MapTutorials"))
      (`self.CreateTutorialMessage` _outrownames_2))
    (:`L_Tutorial`
      (if (== (`self.CombatTutorialCounter`) 0)
        (bind _outrownames_3 (`DataTableFunctionLibrary.GetDataTableRowNames` "/Game/Data/DT_CombatTutorials.DT_CombatTutorials"))
        (`self.CreateTutorialMessage` _outrownames_3)
        (else
          (bind _outrownames_4 (`DataTableFunctionLibrary.GetDataTableRowNames` "/Game/Data/DT_RewardTutorials.DT_RewardTutorials"))
          (`self.CreateTutorialMessage` _outrownames_4))))
    (:`L_NoncombatEncounter`
      (bind _outrownames_5 (`DataTableFunctionLibrary.GetDataTableRowNames` "/Game/Data/DT_EventTutorials.DT_EventTutorials" :!label _label))
      (`self.CreateTutorialMessage` _outrownames_5))
    (:`L_NonCombatArt`
      (goto _label))
    (:`L_NonCombatArtNight`
      (goto _label))))