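; Turn-based 4x4 grid arena pawn that takes possession, spawns a player and enemy in opposite corners, and runs their turns.
; Child-actor tiles form a flat array with a parallel occupancy array, used to highlight free orthogonal neighbours.
; Clicking moves the current combatant to the traced tile without a walkability check, while enemies pick a random walkable tile.
; EndCurrentTurn cycles combatants but is not called here; look input orbits the spring arm.
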(event `self.ReceiveBeginPlay`
  (`self.ChangePlayerPossession`)
  (set `PlayerController.bShowMouseCursor` true (`GameplayStatics.GetPlayerController` 0))
  (`self.InitialiseGame`)
  (`self.UpdateOccupiedTiles`)
  (`self.StartPlayersTurn`))

(event `EnhancedInput|/Game/Inputs/InputActions/IA_LookAround`
  (params (ActionValue :type "Vector2D Structure") (ElapsedSeconds :type "Float (double-precision)") (TriggeredSeconds :type "Float (double-precision)") (InputAction :type "InputAction Object Reference" :default "/Game/Inputs/InputActions/IA_LookAround.IA_LookAround"))
  (bind (_x _y) (`KismetMathLibrary.BreakVector2D` ActionValue))
  ;[1 1 1 0.5 30] Inputs
  (:`Triggered`
    (`SceneComponent.K2_SetWorldRotation` (`self.SpringArm`) (`KismetMathLibrary.MakeRotator` 0.0 (`KismetMathLibrary.FClamp` (+ _y (.pitch (`SceneComponent.K2_GetComponentRotation` (`self.SpringArm`)))) -70.0 10.0) (+ (.yaw (`SceneComponent.K2_GetComponentRotation` (`self.SpringArm`))) _x)) false false)))

(event `EnhancedInput|/Game/Inputs/InputActions/IA_Interact`
  (params (ActionValue :type Boolean) (ElapsedSeconds :type "Float (double-precision)") (TriggeredSeconds :type "Float (double-precision)") (InputAction :type "InputAction Object Reference" :default "/Game/Inputs/InputActions/IA_Interact.IA_Interact"))
  (bind (_hitresult _returnvalue) (`PlayerController.GetHitResultUnderCursorByChannel` (`GameplayStatics.GetPlayerController` 0) "TraceTypeQuery1" true))
  (:`Started`
    (if _returnvalue
      (bind _asbp_tile (cast `/Game/Blueprints/BP_Tile` (`.HitActor` (`GameplayStatics.BreakHitResult` _hitresult))))
      (`/Game/Blueprints/BP_Tile.ChangeMat` _asbp_tile "/Game/Materials/M_TileGold.M_TileGold")
      (bind _tileindex (`self.FindTilesIndex` _asbp_tile))
      (`/Game/Blueprints/BP_Entity.MoveToTile` (`self.CurrentCombatantsTurn`) _tileindex)
      (`self.ResetAllTileColour`)
      (`self.UpdateOccupiedTiles`)
      (`self.UpdateWalkableTiles`))))

(fn `ChangePlayerPossession`
  (bind _returnvalue (`GameplayStatics.GetPlayerController` 0))
  (`PlayerController.SetViewTargetWithBlend` _returnvalue self 0.0 "VTBlend_Linear" 0.0 false)
  (`Controller.Possess` _returnvalue self)
  (bind _returnvalue_2 (`GameplayStatics.GetActorOfClass` "/Script/Engine.DefaultPawn"))
  (if (`KismetSystemLibrary.IsValid` _returnvalue_2)
    (`self.K2_DestroyActor` _returnvalue_2)))

(fn `ChangeTilesColour`
  (params (TileIndex :type Integer) (Material :type "Material Object Reference"))
  (bind _asbp_tile (cast `/Game/Blueprints/BP_Tile` (`ChildActorComponent.ChildActor` (`|GetArrayItem` (`self.GridArray`) TileIndex))))
  (`/Game/Blueprints/BP_Tile.ChangeMat` _asbp_tile Material))

(fn `EndCurrentTurn`
  (bind _combatants (`self.Combatants`))
  (set `self.CurrentCombatantsTurn` (`|GetArrayItem` (`self.Combatants`) (mod (+ (`KismetArrayLibrary.Array_Find` _combatants (`self.CurrentCombatantsTurn`)) 1) (`KismetArrayLibrary.Array_Length` _combatants))))
  (`self.StartPlayersTurn`))

(fn `FindTilesIndex`
  (params (Tile :type "/Game/Blueprints/BP_Tile Object Reference"))
  (returns (TileIndex :type Integer))
  (for (_array_element _array_index) (`self.GridArray`)
    (bind _asbp_tile (cast `/Game/Blueprints/BP_Tile` (`ChildActorComponent.ChildActor` _array_element)))
    (if (== _asbp_tile Tile)
      (return _array_index))))

(fn `GetTileFromGridCoord`
  (params (X :type Integer) (Y :type Integer))
  (returns (TileOccupied :type Boolean) (Tile :type "/Game/Blueprints/BP_Tile Object Reference") (TileIndex :type Integer))
  (bind _returnvalue (+ X (* Y 4)))
  (bind _asbp_tile (cast `/Game/Blueprints/BP_Tile` (`ChildActorComponent.ChildActor` (`|GetArrayItem` (`self.GridArray`) _returnvalue))))
  (return (`|GetArrayItem` (`self.OccupiedGrid`) _returnvalue) _asbp_tile _returnvalue))

(fn `InitialiseGame`
  (bind _returnvalue (`|SpawnActorFromClass` "/Game/Blueprints/BP_Player.BP_Player_C" (`KismetMathLibrary.MakeTransform` (`SceneComponent.K2_GetComponentLocation` (`|GetArrayItem` (`self.GridArray`)))) "Undefined" "MultiplyWithRoot" null null))
  (`KismetArrayLibrary.Array_Add` (`self.Combatants`) _returnvalue)
  (set `/Game/Blueprints/BP_Entity.CurrentTile` 0 _returnvalue)
  (bind _returnvalue_2 (`|SpawnActorFromClass` "/Game/Blueprints/BP_Enemy.BP_Enemy_C" (`KismetMathLibrary.MakeTransform` (`SceneComponent.K2_GetComponentLocation` (`|GetArrayItem` (`self.GridArray`) 15))) "Undefined" "MultiplyWithRoot" null null))
  (`KismetArrayLibrary.Array_Add` (`self.Combatants`) _returnvalue_2)
  (set `/Game/Blueprints/BP_Entity.CurrentTile` 15 _returnvalue_2)
  (set `self.CurrentCombatantsTurn` _returnvalue))

(fn `ResetAllTileColour`
  (for _array_element (`self.GridArray`)
    (bind _asbp_tile (cast `/Game/Blueprints/BP_Tile` (`ChildActorComponent.ChildActor` _array_element)))
    (`/Game/Blueprints/BP_Tile.ChangeMat` _asbp_tile "/Game/Materials/M_TileRed.M_TileRed")))

(fn `StartPlayersTurn`
  (bind _currentcombatantsturn (`self.CurrentCombatantsTurn`))
  (`self.ResetAllTileColour`)
  (`self.ChangeTilesColour` (`/Game/Blueprints/BP_Entity.CurrentTile` (`self.CurrentCombatantsTurn`)) "/Game/Materials/M_TileGold.M_TileGold")
  (`self.UpdateOccupiedTiles`)
  (`self.UpdateWalkableTiles`)
  (cast `/Game/Blueprints/BP_Player` _currentcombatantsturn
    (:`CastFailed`
      (bind _asbp_enemy (cast `/Game/Blueprints/BP_Enemy` _currentcombatantsturn)
        (:`then`
          (`/Game/Blueprints/BP_Entity.MoveToTile` _asbp_enemy (`|GetArrayItem` (`self.CurrentWalkableTileIndices`) (`KismetMathLibrary.RandomIntegerInRange` 0 (- (`KismetArrayLibrary.Array_Length` (`self.CurrentWalkableTileIndices`)) 1)))))
        (:`CastFailed`
          (`KismetSystemLibrary.PrintString` "Blueprint: BP_newArena, Function: StartPlayersTurn \nSomething went wrong with casting current combatant"))))))

(fn `UpdateOccupiedTiles`
  (for (_ _array_index) (`self.OccupiedGrid`)
    (`KismetArrayLibrary.Array_Set` (`self.OccupiedGrid`) _array_index))
  (for _array_element (`self.Combatants`)
    (`KismetArrayLibrary.Array_Set` (`self.OccupiedGrid`) (`/Game/Blueprints/BP_Entity.CurrentTile` _array_element) true)))

(fn `UpdateWalkableTiles`
  (locals (XCoord :type Integer) (yCoord :type Integer))
  (bind _currenttile (`/Game/Blueprints/BP_Entity.CurrentTile` (`self.CurrentCombatantsTurn`)))
  (`KismetArrayLibrary.Array_Clear` (`self.CurrentWalkableTileIndices`))
  (set `local.XCoord` (mod _currenttile 4))
  (set `local.yCoord` (`KismetMathLibrary.FTrunc` (/ (`KismetMathLibrary.Conv_IntToDouble` _currenttile) 4.0)))
  (`|ExecutionSequence`
    (:`then_0`
      (if (> (`local.XCoord`) 0)
        (bind (_tileoccupied _tile _tileindex) (`self.GetTileFromGridCoord` (- (`local.XCoord`) 1) (`local.yCoord`)))
        (if (not _tileoccupied)
          (`/Game/Blueprints/BP_Tile.ChangeMat` _tile "/Game/Materials/M_TileGreen.M_TileGreen")
          (`KismetArrayLibrary.Array_Add` (`self.CurrentWalkableTileIndices`) _tileindex))))
    (:`then_1`
      (if (< (`local.XCoord`) 3)
        (bind (_tileoccupied_2 _tile_2 _tileindex_2) (`self.GetTileFromGridCoord` (+ (`local.XCoord`) 1) (`local.yCoord`)))
        (if (not _tileoccupied_2)
          (`/Game/Blueprints/BP_Tile.ChangeMat` _tile_2 "/Game/Materials/M_TileGreen.M_TileGreen")
          (`KismetArrayLibrary.Array_Add` (`self.CurrentWalkableTileIndices`) _tileindex_2))))
    (:`then_2`
      (if (> (`local.yCoord`) 0)
        (bind (_tileoccupied_3 _tile_3 _tileindex_3) (`self.GetTileFromGridCoord` (`local.XCoord`) (- (`local.yCoord`) 1)))
        (if (not _tileoccupied_3)
          (`/Game/Blueprints/BP_Tile.ChangeMat` _tile_3 "/Game/Materials/M_TileGreen.M_TileGreen")
          (`KismetArrayLibrary.Array_Add` (`self.CurrentWalkableTileIndices`) _tileindex_3))))
    (:`then_3`
      (if (< (`local.yCoord`) 3)
        (bind (_tileoccupied_4 _tile_4 _tileindex_4) (`self.GetTileFromGridCoord` (`local.XCoord`) (+ (`local.yCoord`) 1)))
        (if (not _tileoccupied_4)
          (`/Game/Blueprints/BP_Tile.ChangeMat` _tile_4 "/Game/Materials/M_TileGreen.M_TileGreen")
          (`KismetArrayLibrary.Array_Add` (`self.CurrentWalkableTileIndices`) _tileindex_4))))))

(fn `UserConstructionScript`
  (set `self.GridArray` (`|MakeArray` (`self.BP_Tile3`) (`self.BP_Tile1`) (`self.BP_Tile15`) (`self.BP_Tile9`) (`self.BP_Tile2`) (`self.BP_Tile`) (`self.BP_Tile8`) (`self.BP_Tile10`) (`self.BP_Tile6`) (`self.BP_Tile4`) (`self.BP_Tile13`) (`self.BP_Tile11`) (`self.BP_Tile5`) (`self.BP_Tile7`) (`self.BP_Tile12`) (`self.BP_Tile14`)))
  (set `self.OccupiedGrid` (`|MakeArray` false false false false false false false false false false false false false false false false)))