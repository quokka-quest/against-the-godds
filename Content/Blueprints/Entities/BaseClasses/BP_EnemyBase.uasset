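; Base enemy for turn-based combat, with a world-space healthbar that turns to face the player camera every tick.
; Turn start activates effects, determines a player target and movement, then queues the turn end to the combat game mode.
; Moves and turn end share the turn event queue: moves carry start and end positions as instanced structs, lerp on a Timeline, and mark themselves complete when finished.
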(event `self.ReceiveBeginPlay`
  (bind _asbp_combat_game_mode (cast `/Game/Blueprints/GameModes/BP_CombatGameMode` (`GameplayStatics.GetGameMode`)))
  (set `self.GameModeRef` _asbp_combat_game_mode)
  (bind _aswb_healthbar (cast `/Game/UI/WB_Healthbar` (`WidgetComponent.GetWidget` (`self.HealthWidget`))))
  (`/Game/UI/WB_Healthbar.Initialise` _aswb_healthbar self))

(event `self.ReceiveTick`
  (params (DeltaSeconds :type "Float (single-precision)"))
  (`parent.ReceiveTick` DeltaSeconds)
  (`self.UpdateHealthbarRot`))

(event `self.SetupTurnStart`
  (`self.ActivateStartOfTurnEffects`)
  (`self.DeterminePlayerTarget`)
  (`self.DetermineMovement`)
  (`self.OnTurnEnd`))

(event `self.OnTurnEnd`
  (`EventQueueBlueprintHandler.EnqueueEvent` (delegate `EnqueueTurnEnd`) (struct) (`self.TurnQueueName`) "None" 0 1))

(event `EnqueueTurnEnd`
  (params (Payload :type "InstancedStruct Structure"))
  (`CombatManager.EndCurrentTurn` (`self.GameModeRef`))
  (`EventQueueSystem.MarkEventAsComplete` (subsystem `EventQueueSystem`) (`self.TurnQueueName`)))

(event `self.EnqueueMovement`
  (params (StartPos :type "Vector Structure") (EndPos :type "Vector Structure"))
  (bind _returnvalue (`BlueprintInstancedStructLibrary.MakeInstancedStruct` (make `/Game/EnumsAndStructs/S_MoveVectors` StartPos EndPos)))
  (`EventQueueBlueprintHandler.EnqueueEvent` (delegate `MovePos`) _returnvalue (`self.TurnQueueName`) "None" 0 1))

(event `MovePos`
  (params (Payload :type "InstancedStruct Structure"))
  (bind _value (`BlueprintInstancedStructLibrary.GetInstancedStructValue` Payload)
    (:`Valid`
      (bind (_direction _newtrack_0) (`Timeline|Timeline` :!via `PlayFromStart`)
        (:`Update`
          (bind (_startpos _targetpos) (break `/Game/EnumsAndStructs/S_MoveVectors` _value))
          (`self.K2_SetActorLocation` (`KismetMathLibrary.VLerp` _startpos _targetpos _newtrack_0)))
        (:`Finished`
          (`EventQueueSystem.MarkEventAsComplete` (subsystem `EventQueueSystem`) (`self.TurnQueueName`)))))))

(fn `UpdateHealthbarRot`
  (`SceneComponent.K2_SetWorldRotation` (`self.HealthWidget`) (`KismetMathLibrary.FindLookAtRotation` (`SceneComponent.K2_GetComponentLocation` (`self.HealthWidget`)) (`PlayerCameraManager.GetCameraLocation` (`GameplayStatics.GetPlayerCameraManager` 0))) false false))

(fn `UserConstructionScript`)