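; Base player combatant for turn-based grid combat, handling turns, death, combat UI updates and a camera-facing health bar.
; Rotations and cell moves run as timelines on a movement event queue, which toggles ability buttons and can apply an ability on arrival.
; Grow and shrink events resize the base plate and update grid occupancy between 2x2 and 1x1.
; ApplyRelics turns the game manager's relics into tagged gameplay effects.
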(event `self.ReceiveBeginPlay`
  (bind _returnvalue (subsystem `EventQueueSystem`))
  ;[0 1 0 0.5 40] Begin and Tick
  (`self.SetRefVariables`)
  (add `EventQueueSystem.OnQueueFinished` _returnvalue (delegate `OnMoveFinished`))
  (add `EventQueueSystem.OnEventQueued` _returnvalue (delegate `OnMoveStarted`)))

(event `self.OnEntityDeath`
  ;[0.15 0 0 0.5 40] On Death Events (Everything that runs immediately on death)
  (`KismetSystemLibrary.Delay` 0.1)
  (`parent.OnEntityDeath`)
  (`SceneComponent.SetVisibility` (`self.BasePlateMesh`) false true)
  (bind _foundwidgets (`WidgetBlueprintLibrary.GetAllWidgetsOfClass` "/Game/UI/Combat/WB_CombatUI.WB_CombatUI_C"))
  (`/Game/UI/Combat/WB_CombatUI.RemoveCombatantOnDeath` (`|GetArrayItem` _foundwidgets) self)
  (if (== (`CombatManager.GetCurrentCombatant` (`self.GameModeRef`)) self)
    (`self.OnTurnEnd`)))

(event `OnMoveFinished`
  (params (QueueTag :type Name))
  ;[0 1 0 0.5 40] Begin and Tick
  (if (== QueueTag (`self.MovementQueue`))
    (bind _foundwidgets (`WidgetBlueprintLibrary.GetAllWidgetsOfClass` "/Game/UI/Combat/WB_PlayerTurnUI.WB_PlayerTurnUI_C"))
    (`/Game/UI/Combat/WB_PlayerTurnUI.ToggleAbilityButtons` (`|GetArrayItem` _foundwidgets) true)))

(event `OnMoveStarted`
  (params (QueueTag :type Name))
  ;[0 1 0 0.5 40] Begin and Tick
  (if (== QueueTag (`self.MovementQueue`))
    (bind _foundwidgets (`WidgetBlueprintLibrary.GetAllWidgetsOfClass` "/Game/UI/Combat/WB_PlayerTurnUI.WB_PlayerTurnUI_C"))
    (`/Game/UI/Combat/WB_PlayerTurnUI.ToggleAbilityButtons` (`|GetArrayItem` _foundwidgets) false)))

(event `self.ReceiveTick`
  (params (DeltaSeconds :type "Float (single-precision)"))
  ;[0 1 0 0.5 40] Begin and Tick
  (`parent.ReceiveTick` DeltaSeconds)
  (`self.UpdateHealthbarRot`))

(event `self.EnqueueRotation`
  (params (StartYaw :type "Float (single-precision)") (EndYaw :type "Float (single-precision)"))
  ;[0 0 1 0.5 40] Rotation Function
  (bind _returnvalue (`BlueprintInstancedStructLibrary.MakeInstancedStruct` (make `/Game/EnumsAndStructs/S_Rotators` StartYaw EndYaw)))
  (`EventQueueBlueprintHandler.EnqueueEvent` (delegate `DoRotation`) _returnvalue (`self.MovementQueue`) "None" 0 1))

(event `self.EnqueueMovement`
  (params (StartPos :type "Vector Structure") (EndPos :type "Vector Structure") (AbilityTrigggered :type "GameplayAbilityBase Class Reference"))
  ;[0 0 1 0.5 40] Cell to Cell Movement Function
  (bind _returnvalue (`BlueprintInstancedStructLibrary.MakeInstancedStruct` (make `/Game/EnumsAndStructs/S_MoveVectors` StartPos EndPos AbilityTrigggered)))
  (`EventQueueBlueprintHandler.EnqueueEvent` (delegate `MovePos`) _returnvalue (`self.MovementQueue`) "None" 0 1))

(event `DoRotation`
  (params (Payload :type "InstancedStruct Structure"))
  ;[0 0 1 0.5 40] Rotation Function
  (bind _value (`BlueprintInstancedStructLibrary.GetInstancedStructValue` Payload)
    (:`Valid`
      (bind (_direction _newtrack_0) (`Timeline|Timeline` :!via `PlayFromStart`)
        (:`Update`
          (bind (_fromyaw _toyaw) (break `/Game/EnumsAndStructs/S_Rotators` _value))
          (`SceneComponent.K2_SetWorldRotation` (`self.BasePlateMesh`) (`KismetMathLibrary.MakeRotator` 0.0 0.0 (`self.ActualRotLerp` _fromyaw _toyaw _newtrack_0)) false false))
        (:`Finished`
          (`EventQueueSystem.MarkEventAsComplete` (subsystem `EventQueueSystem`) (`self.MovementQueue`)))))))

(event `MovePos`
  (params (Payload :type "InstancedStruct Structure"))
  ;[0 0 1 0.5 40] Cell to Cell Movement Function
  (bind _value (`BlueprintInstancedStructLibrary.GetInstancedStructValue` Payload)
    (:`Valid`
      (bind (_direction _newtrack_0) (`Timeline|MoveTimeLine` :!via `PlayFromStart`)
        (:`Update`
          (bind (_startpos _targetpos _membervar_5) (break `/Game/EnumsAndStructs/S_MoveVectors` _value))
          (`self.K2_SetActorLocation` (`KismetMathLibrary.VLerp` _startpos _targetpos _newtrack_0)))
        (:`Finished`
          (if (`KismetSystemLibrary.IsValidClass` _membervar_5)
            (`/Game/Blueprints/BP_CellEffectActivator.ApplyAbilityToTarget` (`self.CellEffectRef`) _membervar_5 self))
          (`EventQueueSystem.MarkEventAsComplete` (subsystem `EventQueueSystem`) (`self.MovementQueue`)))))))

(event `Grow2x2`
  (params (Size :type "GridData Structure") (PatternRotation :type "EPatternRotation Enum" :default "R0"))
  (bind _baseplatemesh (`self.BasePlateMesh`))
  ;[0 0.1 0.15 0.5 40] Ability Anims
  (set `self.RotationSweep` Size)
  (set `self.EntityRotations` (`|MakeMap` "R0" Size "R90" Size "R180" Size "R270" Size :!type "EPatternRotation Enum"))
  (`SceneComponent.SetWorldScale3D` _baseplatemesh (2.5 2.5 2.5))
  (`SceneComponent.K2_SetRelativeLocation` _baseplatemesh (`BlueprintMapLibrary.Map_Find` (`self.RotationOffsetMap`) PatternRotation) false false)
  (`CombatManager.ChangeEntitysOccupancy` (`self.GameModeRef`) self false))

(event `self.SetupTurnStart`
  ;[0 1 1 0.5 40] On Turn Start: everything to happen at the beginning of this entities turn
  (`self.ActivateStartOfTurnEffects`)
  (if (not (`self.HasEntityDied`))
    (bind _foundwidgets (`WidgetBlueprintLibrary.GetAllWidgetsOfClass` "/Game/UI/Combat/WB_PlayerTurnUI.WB_PlayerTurnUI_C"))
    (bind _output (`|GetArrayItem` _foundwidgets))
    (`/Game/UI/Combat/SubWidgets/WBP_AttackMenu.UpdateAbilities` (`/Game/UI/Combat/WB_PlayerTurnUI.WBP_AttackMenu` _output) self)
    (`/Game/UI/Combat/WB_PlayerTurnUI.ToggleAbilityButtons` _output true)))

(event `ShrinkTo1x1`
  (params (Size :type "GridData Structure") (PatternRotation :type "EPatternRotation Enum" :default "R0"))
  (bind _baseplatemesh (`self.BasePlateMesh`))
  ;[0 0.1 0.15 0.5 40] Ability Anims
  (`CombatManager.ChangeEntitysOccupancy` (`self.GameModeRef`) self true)
  (set `self.RotationSweep` Size)
  (set `self.EntityRotations` (`|MakeMap` "R0" Size "R90" Size "R180" Size "R270" Size :!type "EPatternRotation Enum"))
  (`SceneComponent.SetWorldScale3D` _baseplatemesh (1.0 1.0 1.0))
  (`SceneComponent.K2_SetRelativeLocation` _baseplatemesh (0.0 0.0 0.0) false false)
  (`CombatManager.ChangeEntitysOccupancy` (`self.GameModeRef`) self false))

(event `self.OnTurnEnd`
  ;[1 0 1 0.5 40] On Turn End: everything to happen when the turn is ended
  (`|ExecutionSequence`
    (:`then_0`
      (bind _foundwidgets (`WidgetBlueprintLibrary.GetAllWidgetsOfClass` "/Game/UI/Combat/WB_PlayerTurnUI.WB_PlayerTurnUI_C"))
      (`/Game/UI/Combat/WB_PlayerTurnUI.ToggleAbilityButtons` (`|GetArrayItem` _foundwidgets) false))
    (:`then_1`
      (`EventQueueBlueprintHandler.EnqueueEvent` (delegate `EnqueueTurnEnd`) (struct) (`self.QueueName`) "None" 0 1))))

(event `self.AbilitySystemComponent.OnFinalStackRemoved`
  (params (EffectClass :type "GameplayEffect Class Reference") (InstantEffectClass :type "GameplayEffect Class Reference"))
  ;[0 0.1 0.15 0.5 40] Ability Anims
  (if (== EffectClass null)
    (`self.ShrinkTo1x1` (struct))))

(event `EnqueueTurnEnd`
  (params (Payload :type "InstancedStruct Structure"))
  ;[1 0 1 0.5 40] On Turn End: everything to happen when the turn is ended
  (`CombatManager.EndCurrentTurn` (`self.GameModeRef`))
  (`EventQueueSystem.MarkEventAsComplete` (subsystem `EventQueueSystem`) (`self.QueueName`)))

(fn `ActualRotLerp`
  (params (From :type "Float (double-precision)") (To :type "Float (double-precision)") (Alpha :type "Float (double-precision)"))
  (returns (Output :type "Float (double-precision)"))
  (locals (FromRot :type "Float (double-precision)") (ToRot :type "Float (double-precision)"))
  (set `local.FromRot` From)
  (set `local.ToRot` To)
  (`|ExecutionSequence`
    (:`then_0`
      (if (== (`KismetMathLibrary.Abs` (- (`local.FromRot`) (`local.ToRot`))) 270.0)
        (if (== (`local.FromRot`) 270.0)
          (set `local.FromRot` -90.0)
          (else
            (set `local.ToRot` -90.0)))))
    (:`then_1`
      (return (`KismetMathLibrary.Lerp` (`local.FromRot`) (`local.ToRot`) (`local.Alpha`))))))

(fn `ApplyRelics`
  (bind _abilitysystemcomponent (`self.AbilitySystemComponent`))
  (bind _abilitysystemcomponent_2 (`self.AbilitySystemComponent`))
  (bind _abilitysystemcomponent_3 (`self.AbilitySystemComponent`))
  (bind _asbp_game_manager (cast `/Game/Blueprints/Managers/BP_GameManager` (`GameplayStatics.GetGameInstance`)))
  (for _array_element (`/Game/Blueprints/Managers/BP_GameManager.CurrentRelics` _asbp_game_manager)
    (switch `/Game/System_NCEvent/RelicSystem/ENUM_RelicApplication` (`.ApplicationType_19_98AE2CE44AB92B246D1127A35366B436` (break `/Game/System_NCEvent/RelicSystem/ST_RelicRow` _array_element))
      (:`NewEnumerator0`
        (bind _returnvalue (`AbilitySystemBlueprintLibrary.AddAssetTag` (`AbilitySystemComponent.MakeOutgoingSpec` :`self` _abilitysystemcomponent_3 :`GameplayEffectClass` (`.GameplayEffect_14_A1B76996459442DE2A1790B702D9CA33` (break `/Game/System_NCEvent/RelicSystem/ST_RelicRow` _array_element))) (struct :`TagName` "Effect.EndOfCombat")))
        (`AbilitySystemComponent.BP_ApplyGameplayEffectSpecToSelf` _abilitysystemcomponent_3 _returnvalue))
      (:`NewEnumerator1`
        (bind _returnvalue_2 (`AbilitySystemBlueprintLibrary.AddAssetTag` (`AbilitySystemComponent.MakeOutgoingSpec` :`self` _abilitysystemcomponent_2 :`GameplayEffectClass` (`.GameplayEffect_14_A1B76996459442DE2A1790B702D9CA33` (break `/Game/System_NCEvent/RelicSystem/ST_RelicRow` _array_element))) (struct :`TagName` "Effect.StartOfTurn")))
        (`TurnBasedAbilitySystemComponent.BindGameplayEffectToOnStackLoss` _abilitysystemcomponent_2 _returnvalue_2 (`AbilitySystemComponent.MakeOutgoingSpec` :`self` (`self.AbilitySystemComponent`) :`GameplayEffectClass` (`.OnStackChange_22_505B09054FA14FBAA16415B9EDA14EC1` (break `/Game/System_NCEvent/RelicSystem/ST_RelicRow` _array_element))) true))
      (:`NewEnumerator2`
        (if (`KismetSystemLibrary.IsValidClass` (`.GameplayEffect_14_A1B76996459442DE2A1790B702D9CA33` (break `/Game/System_NCEvent/RelicSystem/ST_RelicRow` _array_element)))
          (bind _returnvalue_3 (`AbilitySystemBlueprintLibrary.AddAssetTag` (`AbilitySystemComponent.MakeOutgoingSpec` :`self` _abilitysystemcomponent :`GameplayEffectClass` (`.GameplayEffect_14_A1B76996459442DE2A1790B702D9CA33` (break `/Game/System_NCEvent/RelicSystem/ST_RelicRow` _array_element))) (struct :`TagName` "Effect.EndOfCombat")))
          (`AbilitySystemComponent.BP_ApplyGameplayEffectSpecToSelf` _abilitysystemcomponent _returnvalue_3))))))

(fn `SetRefVariables`
  (bind _asbp_combat_game_mode (cast `/Game/Blueprints/GameModes/BP_CombatGameMode` (`GameplayStatics.GetGameMode`)))
  (set `self.GameModeRef` _asbp_combat_game_mode)
  (bind _asbp_player_pawn (cast `/Game/Blueprints/BP_PlayerPawn` (`GameplayStatics.GetPlayerPawn` 0)))
  (set `self.PlayerPawnRef` _asbp_player_pawn)
  (bind _returnvalue (`GameplayStatics.GetActorOfClass` "/Game/Blueprints/BP_CellEffectActivator.BP_CellEffectActivator_C"))
  (set `self.CellEffectRef` _returnvalue)
  (`EventQueueSystem.CreateQueue` (subsystem `EventQueueSystem`) (`self.MovementQueue`) false)
  (bind _aswb_health_bar (cast `/Game/UI/Combat/SubWidgets/WB_HealthBar` (`WidgetComponent.GetWidget` (`self.HealthWidget`))))
  (`/Game/UI/Combat/SubWidgets/WB_HealthBar.InitialiseHealthBar` _aswb_health_bar self))

(fn `UpdateHealthbarRot`
  (`SceneComponent.K2_SetWorldRotation` (`self.HealthWidget`) (`KismetMathLibrary.FindLookAtRotation` (`SceneComponent.K2_GetComponentLocation` (`self.HealthWidget`)) (`PlayerCameraManager.GetCameraLocation` (`GameplayStatics.GetPlayerCameraManager` 0))) false false))

(fn `UserConstructionScript`)