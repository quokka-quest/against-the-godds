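; BP_PoisonShroom is an enemy Blueprint for a poison mushroom that drives its animations.
; On BeginPlay it calls the parent and caches its skeletal mesh's anim instance as ABP_Shroom.
; Animation events forward to that instance: attack and damaged call its functions, while death and win set boolean flags on it.
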(event `self.ReceiveBeginPlay`
  (`parent.ReceiveBeginPlay`)
  (set `self.AnimRef` (cast `/Game/Blueprints/Animations/ABP_Shroom` (`SkeletalMeshComponent.GetAnimInstance` (`self.SkeletalMesh`)) :!pure true)))

(event `self.PlayAttackAnim`
  (`/Game/Blueprints/Animations/ABP_Shroom.PlayAttackAnim` (`self.AnimRef`)))

(event `self.PlayDamagedAnim`
  (`/Game/Blueprints/Animations/ABP_Shroom.PlayDamagedAnim` (`self.AnimRef`)))

(event `self.PlayDeathAnim`
  (set `/Game/Blueprints/Animations/ABP_Shroom.PlayDeath` true (`self.AnimRef`)))

(event `self.PlayWinAnim`
  (set `/Game/Blueprints/Animations/ABP_Shroom.PlayWin` true (`self.AnimRef`)))

(fn `UserConstructionScript`
  (`parent.UserConstructionScript`))