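; BP_Wolf_White is a white wolf enemy that connects its parent class's animation events to the wolf Animation Blueprint.
; BeginPlay runs the parent logic, then casts the skeletal mesh's anim instance to ABP_Wolf and caches it.
; The attack event calls PlayAttackAnim on that instance, while the death and win events set its PlayDeath and PlayWin flags.
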(event `self.ReceiveBeginPlay`
  (`parent.ReceiveBeginPlay`)
  (set `self.AnimRef` (cast `/Game/Blueprints/Animations/ABP_Wolf` (`SkeletalMeshComponent.GetAnimInstance` (`self.SkeletalMesh`)) :!pure true)))

(event `self.PlayAttackAnim`
  (`/Game/Blueprints/Animations/ABP_Wolf.PlayAttackAnim` (`self.AnimRef`)))

(event `self.PlayDeathAnim`
  (set `/Game/Blueprints/Animations/ABP_Wolf.PlayDeath` true (`self.AnimRef`)))

(event `self.PlayWinAnim`
  (set `/Game/Blueprints/Animations/ABP_Wolf.PlayWin` true (`self.AnimRef`)))

(fn `UserConstructionScript`
  (`parent.UserConstructionScript`))