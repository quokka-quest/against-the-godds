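; BP_MagSupport is a player entity Blueprint, a magic support character by its name, that drives animations through the Jester anim Blueprint.
; On BeginPlay it calls the parent and caches the skeletal mesh's anim instance as ABP_Jester.
; Attack, damaged, death and win events set matching play flags on that anim instance.
; A stat update event sends its stats to the game instance.
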(event `self.ReceiveBeginPlay`
  (`parent.ReceiveBeginPlay`)
  (set `self.AnimRef` (cast `/Game/Blueprints/Animations/ABP_Jester` (`SkeletalMeshComponent.GetAnimInstance` (`self.SkeletalMesh`)) :!pure true)))

(event `self.UpdateGlobalStatData`
  (`self.SendStatsToGameInstance` "BP_MagSupport_C"))

(event `self.PlayAttackAnim`
  (set `/Game/Blueprints/Animations/ABP_Jester.PlayAttack` true (`self.AnimRef`)))

(event `self.PlayDamagedAnim`
  (set `/Game/Blueprints/Animations/ABP_Jester.PlayDamaged` true (`self.AnimRef`)))

(event `self.PlayDeathAnim`
  (set `/Game/Blueprints/Animations/ABP_Jester.PlayDeath` true (`self.AnimRef`)))

(event `self.PlayWinAnim`
  (set `/Game/Blueprints/Animations/ABP_Jester.PlayWin` true (`self.AnimRef`)))

(fn `UserConstructionScript`
  (`parent.UserConstructionScript`))