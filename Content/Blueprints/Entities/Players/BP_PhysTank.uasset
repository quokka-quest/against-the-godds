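; BP_PhysTank is a player entity Blueprint that handles the end of a grow effect and reports its stats to the game instance.
; When the last GE_Grow stack is removed from its Ability System Component, it shrinks to a 1x1 footprint.
; It then damages itself for half its current health, rounded up, through a GE_Damage spec using a SetByCaller magnitude.
; The construction script only calls the parent.
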(event `self.UpdateGlobalStatData`
  (`self.SendStatsToGameInstance` "BP_PhysTank_C"))

(event `self.AbilitySystemComponent.OnFinalStackRemoved`
  (params (EffectClass :type "GameplayEffect Class Reference") (InstantEffectClass :type "GameplayEffect Class Reference"))
  (bind _returnvalue (`AbilitySystemBlueprintLibrary.GetAbilitySystemComponent` null))
  (if (== EffectClass "/Game/GAS/Effects/GE_Grow.GE_Grow_C")
    (`self.ShrinkTo1x1` (struct))
    (bind _returnvalue_2 (`AbilitySystemBlueprintLibrary.AssignTagSetByCallerMagnitude` (`AbilitySystemComponent.MakeOutgoingSpec` :`self` _returnvalue :`GameplayEffectClass` "/Game/GAS/Effects/GE_Damage.GE_Damage_C") (struct :`TagName` "Damage.SetByCaller") (`KismetMathLibrary.Conv_IntToDouble` (`KismetMathLibrary.FCeil` (/ (`self.GetCurrentHealth`) 2.0)))))
    (`AbilitySystemComponent.BP_ApplyGameplayEffectSpecToSelf` _returnvalue _returnvalue_2)))

(fn `UserConstructionScript`
  (`parent.UserConstructionScript`))