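; BP_MagTank is the MagTank player entity, a child Blueprint that supplies its own animation and stat hooks to parent logic.
; On BeginPlay it caches its skeletal mesh's ABP_Ram anim instance, then forwards attack and damage events as calls and sets flags for death and win.
; Its UpdateGlobalStatData event sends the tank's stats to the Game Instance.
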(event `self.UpdateGlobalStatData`
  (`self.SendStatsToGameInstance` "BP_MagTank_C"))

(event `self.ReceiveBeginPlay`
  (`parent.ReceiveBeginPlay`)
  (set `self.AnimRef` (cast `/Game/Blueprints/Animations/ABP_Ram` (`SkeletalMeshComponent.GetAnimInstance` (`self.SkeletalMesh`)) :!pure true)))

(event `self.PlayAttackAnim`
  (`/Game/Blueprints/Animations/ABP_Ram.PlayAttackAnim` (`self.AnimRef`)))

(event `self.PlayDamagedAnim`
  (`/Game/Blueprints/Animations/ABP_Ram.PlayDamagedAnim` (`self.AnimRef`)))

(event `self.PlayDeathAnim`
  (set `/Game/Blueprints/Animations/ABP_Ram.PlayDeath` true (`self.AnimRef`)))

(event `self.PlayWinAnim`
  (set `/Game/Blueprints/Animations/ABP_Ram.PlayWin` true (`self.AnimRef`)))

(fn `UserConstructionScript`
  (`parent.UserConstructionScript`))