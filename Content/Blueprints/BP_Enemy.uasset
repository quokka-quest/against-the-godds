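; Turn-based enemy combatant that closes in on the nearest player on the arena's tile grid.
; ExecuteTurn picks the closest BP_Player by mesh distance, steps one tile toward it unless already adjacent (diagonals included), then ends the turn; no attack happens here.
; FinishTurn resets the AI controller's IsTurn and HasMoved blackboard flags.
; InitialiseTurn only calls its parent; the code setting IsTurn is disconnected.
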(fn `DetermineMovement`
  (bind _playerinrange (`self.IsTargetInMeleeRange`))
  (if (not _playerinrange)
    (bind _tileindex (`self.FindTileToMoveTo`))
    (`self.MoveToTile` _tileindex)))

(fn `ExecuteTurn`
  (`self.UpdatePlayerTarget`)
  (`self.DetermineMovement`)
  (`/Game/Blueprints/BP_Arena.EndCurrentTurn` (`self.ArenaRef`)))

(fn `FindTileToMoveTo`
  (returns (TileIndex :type Integer))
  (locals (TargetTileX :type Integer) (TargetTileY :type Integer))
  (bind (_x _y) (`/Game/Blueprints/BP_Arena.GetTileCoordsFromIndex` (`self.ArenaRef`) (`/Game/Blueprints/BP_Entity.CurrentTile` (`self.PriorityTarget`))))
  (set `local.TargetTileX` _x)
  (set `local.TargetTileY` _y)
  (bind (_x_2 _y_2) (`/Game/Blueprints/BP_Arena.GetTileCoordsFromIndex` (`self.ArenaRef`) (`self.CurrentTile`)))
  (bind (_tileoccupied _tile _tileindex) (`/Game/Blueprints/BP_Arena.GetTileFromGridCoord` (`self.ArenaRef`) (+ _x_2 (`KismetMathLibrary.Clamp` (- (`local.TargetTileX`) _x_2) -1 1)) (+ _y_2 (`KismetMathLibrary.Clamp` (- (`local.TargetTileY`) _y_2) -1 1))))
  (return _tileindex))

(fn `FinishTurn`
  (`parent.FinishTurn`)
  (`self.ResetBlackBoard`))

(fn `InitialiseTurn`
  (`parent.InitialiseTurn`))

(fn `IsTargetInMeleeRange`
  (returns (PlayerInRange :type Boolean))
  (locals (Xcoord :type Integer) (YCoord :type Integer))
  (bind (_x _y) (`/Game/Blueprints/BP_Arena.GetTileCoordsFromIndex` (`self.ArenaRef`) (`self.CurrentTile`)))
  (set `local.Xcoord` _x)
  (set `local.YCoord` _y)
  (bind (_x_2 _y_2) (`/Game/Blueprints/BP_Arena.GetTileCoordsFromIndex` (`self.ArenaRef`) (`/Game/Blueprints/BP_Entity.CurrentTile` (`self.PriorityTarget`))))
  (return (and (<= (`KismetMathLibrary.Abs_Int` (- _x_2 (`local.Xcoord`))) 1) (<= (`KismetMathLibrary.Abs_Int` (- _y_2 (`local.YCoord`))) 1))))

(fn `ResetBlackBoard`
  (locals (BlackBoard :type "BlackboardComponent Object Reference"))
  (bind _asaic_enemy_controller (cast `/Game/AI/AIC_EnemyController` (`AIBlueprintHelperLibrary.GetAIController` self)))
  (set `local.BlackBoard` (`AIBlueprintHelperLibrary.GetBlackboard` _asaic_enemy_controller))
  (`BlackboardComponent.SetValueAsBool` (`local.BlackBoard`) "IsTurn" false)
  (`BlackboardComponent.SetValueAsBool` (`local.BlackBoard`) "HasMoved" false))

(fn `UpdatePlayerTarget`
  (locals (XCoord :type Integer) (YCoord :type Integer) (ClosestPlayer :type "/Game/Blueprints/BP_Player Object Reference") (SmallestDist :type "Float (double-precision)" :default 1000000.0))
  (for _array_element (`/Game/Blueprints/BP_Arena.Combatants` (`self.ArenaRef`))
    (bind _asbp_player (cast `/Game/Blueprints/BP_Player` _array_element))
    (bind _returnvalue (`KismetMathLibrary.VSize` (- (`SceneComponent.K2_GetComponentLocation` (`/Game/Blueprints/BP_Entity.Mesh` _asbp_player)) (`SceneComponent.K2_GetComponentLocation` (`self.Mesh`)))))
    (if (< _returnvalue (`local.SmallestDist`))
      (set `local.SmallestDist` _returnvalue)
      (set `local.ClosestPlayer` _asbp_player)))
  (set `self.PriorityTarget` (`local.ClosestPlayer`)))

(fn `UserConstructionScript`
  (`parent.UserConstructionScript`))