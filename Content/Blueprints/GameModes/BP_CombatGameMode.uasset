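; Game mode for turn-based grid combat, handling encounter setup, turn handover and win/lose screens.
; BeginPlay creates the turn queue, sets input, applies game-mode relics, then enqueues spawning, initiative rolls with player relics, combat UI, dead-player removal and first turn.
; Queued events mark themselves complete; turn end notifies the UI and enqueues the next turn.
; Victory opens dice upgrades; a helper maps source-to-target offset to an eight-direction knockback entry.
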(event `self.ReceiveBeginPlay`
  ;[0 1 0 0.5 60] Start of Combat logic
  (`self.OnCombatStarted`)
  (`self.CheckGMRelics`)
  (`KismetSystemLibrary.Delay` 0.1)
  (`GridManagerTool.ResetHighlights` (`self.GridManager`))
  (`EventQueueBlueprintHandler.EnqueueEvent` (delegate `EnqueuePlayerSpawn`) (struct) "None" "None" 0 1)
  (`EventQueueBlueprintHandler.EnqueueEvent` (delegate `EnqueueEnemySpawn`) (struct) (`self.TurnEventQueueName`) "None" 0 1)
  (`EventQueueBlueprintHandler.EnqueueEvent` (delegate `EnqueueInitiativeRoles`) (struct) (`self.TurnEventQueueName`) "None" 0 1)
  (`EventQueueBlueprintHandler.EnqueueEvent` (delegate `EnableCombatUI`) (struct) (`self.TurnEventQueueName`) "None" 0 1)
  (`EventQueueBlueprintHandler.EnqueueEvent` (delegate `EnqueuPlayerCheck`) (struct) (`self.TurnEventQueueName`) "None" 0 1)
  (`EventQueueBlueprintHandler.EnqueueEvent` (delegate `EnqueueFirstTurnStart`) (struct) (`self.TurnEventQueueName`) "None" 0 1))

(event `EnableCombatUI`
  (params (Payload :type "InstancedStruct Structure"))
  ;[0 1 0 0.5 60] Start of Combat logic
  (bind _returnvalue (`|CreateWidget` "/Game/UI/Combat/WB_CombatUI.WB_CombatUI_C"))
  (`UserWidget.AddToViewport` _returnvalue 0)
  (`/Game/UI/Combat/WB_CombatUI.InitialiseCombatEncounter` _returnvalue)
  (`EventQueueSystem.MarkEventAsComplete` (subsystem `EventQueueSystem`) (`self.TurnEventQueueName`)))

(event `EnqueueEnemySpawn`
  (params (Payload :type "InstancedStruct Structure"))
  ;[0 1 0 0.5 60] Start of Combat logic
  (`self.SpawnEnemies`)
  (`EventQueueSystem.MarkEventAsComplete` (subsystem `EventQueueSystem`) (`self.TurnEventQueueName`)))

(event `EnqueueFirstTurnStart`
  (params (Payload :type "InstancedStruct Structure"))
  ;[0 1 0 0.5 60] Start of Combat logic
  (`self.StartCurrentTurn`)
  (`EventQueueSystem.MarkEventAsComplete` (subsystem `EventQueueSystem`) (`self.TurnEventQueueName`)))

(event `EnqueuePlayerSpawn`
  (params (Payload :type "InstancedStruct Structure"))
  ;[0 1 0 0.5 60] Start of Combat logic
  (`self.SpawnPlayerCharacters`)
  (`EventQueueSystem.MarkEventAsComplete` (subsystem `EventQueueSystem`) (`self.TurnEventQueueName`)))

(event `EnqueueInitiativeRoles`
  (params (Payload :type "InstancedStruct Structure"))
  ;[0 1 0 0.5 60] Start of Combat logic
  (`self.RollDiceForInitiative`)
  (`EventQueueSystem.MarkEventAsComplete` (subsystem `EventQueueSystem`) (`self.TurnEventQueueName`))
  (bind _outactors (`GameplayStatics.GetAllActorsOfClass` "/Game/Blueprints/Entities/BaseClasses/BP_PlayerBase.BP_PlayerBase_C"))
  (for _array_element _outactors
    (`/Game/Blueprints/Entities/BaseClasses/BP_PlayerBase.ApplyRelics` _array_element)))

(event `EnqueuPlayerCheck`
  (params (Payload :type "InstancedStruct Structure"))
  ;[0 1 0 0.5 60] Start of Combat logic
  (`self.RemoveDeadPlayers`)
  (`EventQueueSystem.MarkEventAsComplete` (subsystem `EventQueueSystem`) (`self.TurnEventQueueName`)))

(event `self.OnPlayersWin`
  ;[0.15 0 0 0.5 40] Player Win and Lost events
  (bind _foundwidgets (`WidgetBlueprintLibrary.GetAllWidgetsOfClass` "/Game/UI/Combat/WB_PlayerTurnUI.WB_PlayerTurnUI_C"))
  (`/Game/UI/Combat/WB_PlayerTurnUI.ToggleAbilityButtons` (`|GetArrayItem` _foundwidgets) false)
  (bind _returnvalue (`|CreateWidget` "/Game/UI/MenuScreens/WB_BattleWon.WB_BattleWon_C"))
  (`UserWidget.AddToViewport` _returnvalue 0)
  (bind _returnvalue_2 (`|CreateWidget` "/Game/UI/DiceUpgrades/WBP_UpgradeDiceScreen.WBP_UpgradeDiceScreen_C"))
  (`UserWidget.AddToViewport` _returnvalue_2 0)
  (`/Game/UI/DiceUpgrades/WBP_UpgradeDiceScreen.StartUpgrades` _returnvalue_2 (`self.UpgradePoints`)))

(event `self.OnPlayersLost`
  ;[0.15 0 0 0.5 40] Player Win and Lost events
  (bind _returnvalue (`|CreateWidget` "/Game/UI/MenuScreens/WB_BattleLost.WB_BattleLost_C"))
  (`UserWidget.AddToViewport` _returnvalue 0))

(event `self.BlueprintEndTurnEvents`
  ;[0 0 1 0.5 40] Blueprint-specific end of turn Logic (for interacting with UI and using the queue subsystem
  (bind _foundwidgets (`WidgetBlueprintLibrary.GetAllWidgetsOfClass` "/Game/UI/Combat/WB_CombatUI.WB_CombatUI_C"))
  (`/Game/UI/Combat/WB_CombatUI.OnCombatantTurnEnd` (`|GetArrayItem` _foundwidgets) (`self.HasRoundEnded`) (`self.CurrentTurnCombatant`))
  (`EventQueueBlueprintHandler.EnqueueEvent` (delegate `StartTheNextTurn`) (struct) (`self.TurnEventQueueName`) "None" 0 1))

(event `StartTheNextTurn`
  (params (Payload :type "InstancedStruct Structure"))
  ;[0 0 1 0.5 40] Blueprint-specific end of turn Logic (for interacting with UI and using the queue subsystem
  (`self.StartCurrentTurn`)
  (`EventQueueSystem.MarkEventAsComplete` (subsystem `EventQueueSystem`) (`self.TurnEventQueueName`)))

(fn `CheckGMRelics`
  (bind _asbp_game_manager (cast `/Game/Blueprints/Managers/BP_GameManager` (`GameplayStatics.GetGameInstance`)))
  (for _array_element (`/Game/Blueprints/Managers/BP_GameManager.CurrentRelics` _asbp_game_manager)
    (switch `/Game/System_NCEvent/RelicSystem/ENUM_RelicApplication` (`.ApplicationType_19_98AE2CE44AB92B246D1127A35366B436` (break `/Game/System_NCEvent/RelicSystem/ST_RelicRow` _array_element))
      (:`NewEnumerator2`
        (`/Game/Blueprints/AC_RelicLogic.ApplyRelics` (`self.AC_RelicLogic`) (break `/Game/System_NCEvent/RelicSystem/ST_RelicRow` _array_element))))))

(fn `GetKnockbackCheckGrid`
  (params (TargetEntity :type "EntityBase Object Reference") (FromCoord :type "IntVector2 Structure"))
  (returns (KnockbackGrid :type "GridData Structure"))
  (locals (XDiff :type Integer) (YDiff :type Integer))
  (bind (_positioncoord_x _positioncoord_y) (break `IntVector2` (`EntityBase.PositionCoord` TargetEntity)))
  (set `local.XDiff` (- _positioncoord_x FromCoord_X))
  (set `local.YDiff` (- _positioncoord_y FromCoord_Y))
  (if (or (!= (`local.XDiff`) 0) (!= (`local.YDiff`) 0))
    (if (== (`KismetMathLibrary.Abs_Int` (`local.XDiff`)) (`KismetMathLibrary.Abs_Int` (`local.YDiff`)))
      (return (`BlueprintMapLibrary.Map_Find` (`self.KnockbackMap`) (make `IntVector2` (`KismetMathLibrary.SignOfInteger` (`local.XDiff`)) (`KismetMathLibrary.SignOfInteger` (`local.YDiff`)))))
      (elif (> (`KismetMathLibrary.Abs_Int` (`local.XDiff`)) (`KismetMathLibrary.Abs_Int` (`local.YDiff`)))
        (return (`BlueprintMapLibrary.Map_Find` (`self.KnockbackMap`) (make `IntVector2` (`KismetMathLibrary.SignOfInteger` (`local.XDiff`)))))
        (elif (> (`KismetMathLibrary.Abs_Int` (`local.YDiff`)) (`KismetMathLibrary.Abs_Int` (`local.XDiff`)))
          (return (`BlueprintMapLibrary.Map_Find` (`self.KnockbackMap`) (make `IntVector2` 0 (`KismetMathLibrary.SignOfInteger` (`local.YDiff`)))))
          (else
            (`KismetSystemLibrary.PrintString` (`KismetStringLibrary.Concat_StrStr` "Error: BP_CombatGameMode ->GetKnockbackCheckGrid:" " The knockback direction check conditions failed to account for a difference of " (`KismetStringLibrary.Conv_IntToString` (`local.XDiff`)) ", " (`KismetStringLibrary.Conv_IntToString` (`local.YDiff`))) true true (struct :`R` 1.0 :`G` 0.013335 :`B` 5.5e-05 :`A` 1.0))
            (return (`BlueprintMapLibrary.Map_Find` (`self.KnockbackMap`) (make `IntVector2` 1)))))))
    (else
      (`KismetSystemLibrary.PrintString` "Error: BP_CombatGameMode ->GetKnockbackCheckGrid: Tried to knockback where source and target are 0 distance" true true (struct :`R` 1.0 :`B` 0.012959 :`A` 1.0) 4.0)
      (return (`BlueprintMapLibrary.Map_Find` (`self.KnockbackMap`) (make `IntVector2` 1))))))

(fn `OnCombatStarted`
  (bind _returnvalue (pcsubsystem `EnhancedInputLocalPlayerSubsystem` (`GameplayStatics.GetPlayerController` 0)))
  (`EventQueueSystem.CreateQueue` (subsystem `EventQueueSystem`) (`self.TurnEventQueueName`) false)
  (`EnhancedInputSubsystemInterface.ClearAllMappings` _returnvalue)
  (`EnhancedInputSubsystemInterface.AddMappingContext` _returnvalue "/Game/Inputs/IMC_InputMap.IMC_InputMap" 0 (struct))
  (`EnhancedInputSubsystemInterface.AddMappingContext` _returnvalue "/Game/Inputs/IMC_PlayersTurn.IMC_PlayersTurn" 0 (struct)))

(fn `UserConstructionScript`)