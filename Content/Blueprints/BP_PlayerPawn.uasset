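; BP_PlayerPawn is the player's pawn for what appears to be a turn-based, tile-based game.
; On BeginPlay it enables the player-turn Enhanced Input context and adds placement and turn UI widgets to the viewport.
; Look input rotates the spring arm with clamped pitch, and interact calls OnTileClick and prints a debug string.
; ToggleTurnInputMapping adds or removes the turn context, while SetTargetTile is an empty stub.
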(event `self.ReceiveBeginPlay`
  (`self.ToggleTurnInputMapping` true)
  (bind _returnvalue (`|CreateWidget` "/Game/UI/WB_PlayerPlacement.WB_PlayerPlacement_C"))
  (`UserWidget.AddToViewport` _returnvalue 0)
  (bind _returnvalue_2 (`|CreateWidget` "/Game/UI/WB_PlayerTurnUI.WB_PlayerTurnUI_C"))
  (`UserWidget.AddToViewport` _returnvalue_2 0))

(event `EnhancedInput|/Game/Inputs/InputActions/IA_LookAround`
  (params (ActionValue :type "Vector2D Structure") (ElapsedSeconds :type "Float (double-precision)") (TriggeredSeconds :type "Float (double-precision)") (InputAction :type "InputAction Object Reference" :default "/Game/Inputs/InputActions/IA_LookAround.IA_LookAround"))
  (bind (_x _y) (`KismetMathLibrary.BreakVector2D` ActionValue))
  ;[1 1 1 0.5 30] Inputs
  (:`Triggered`
    (`SceneComponent.K2_SetWorldRotation` (`self.SpringArm`) (`KismetMathLibrary.MakeRotator` 0.0 (`KismetMathLibrary.FClamp` (+ _y (.pitch (`SceneComponent.K2_GetComponentRotation` (`self.SpringArm`)))) -70.0 10.0) (+ (.yaw (`SceneComponent.K2_GetComponentRotation` (`self.SpringArm`))) _x)) false false)))

(event `EnhancedInput|/Game/Inputs/InputActions/IA_Interact`
  (params (ActionValue :type Boolean) (ElapsedSeconds :type "Float (double-precision)") (TriggeredSeconds :type "Float (double-precision)") (InputAction :type "InputAction Object Reference" :default "/Game/Inputs/InputActions/IA_Interact.IA_Interact"))
  ;[1 1 1 0.5 30] Inputs
  (:`Started`
    (`self.OnTileClick`)
    (`KismetSystemLibrary.PrintString` "Hello")))

(event `self.ToggleTurnInputMapping`
  (params (EnableInputs :type Boolean))
  (if EnableInputs
    (`EnhancedInputSubsystemInterface.AddMappingContext` (pcsubsystem `EnhancedInputLocalPlayerSubsystem` (`GameplayStatics.GetPlayerController` 0)) "/Game/Inputs/IMC_PlayersTurn.IMC_PlayersTurn" 0 (struct))
    (else
      (`EnhancedInputSubsystemInterface.RemoveMappingContext` (pcsubsystem `EnhancedInputLocalPlayerSubsystem` (`GameplayStatics.GetPlayerController` 0)) "/Game/Inputs/IMC_PlayersTurn.IMC_PlayersTurn" (struct)))))

(fn `SetTargetTile`)

(fn `UserConstructionScript`)