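; Player Blueprint that adds a turn UI to its parent's turn-based logic.
; InitialiseTurn runs the parent logic, then creates a WB_PlayerTurnUI widget, stores it, adds it to the viewport and initialises it with a reference to the player.
; FinishTurn runs the parent logic, then removes that widget, so a fresh UI is built for each turn.
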(fn `FinishTurn`
  (`parent.FinishTurn`)
  (`Widget.RemoveFromParent` (`self.UIRef`)))

(fn `InitialiseTurn`
  (`parent.InitialiseTurn`)
  (bind _returnvalue (`|CreateWidget` "/Game/UI/WB_PlayerTurnUI.WB_PlayerTurnUI_C"))
  (bind _output_get (set `self.UIRef` _returnvalue))
  (`UserWidget.AddToViewport` _output_get 0)
  (`/Game/UI/WB_PlayerTurnUI.Initialise` _output_get self))

(fn `UserConstructionScript`
  (`parent.UserConstructionScript`))