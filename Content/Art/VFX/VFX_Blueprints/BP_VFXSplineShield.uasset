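; Spline-driven VFX actor that plays a thrown-shield Niagara effect along a path through a set of target actors.
; SetSplinePoints rebuilds the spline from the actors' world locations, raised slightly above each origin, while counting the points.
; That count looks up lifetime and speed maps to set the Niagara variables for the shield and trail before activating the effect.
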(event `SetSplinePoints`
  (params (ActorArray :type "Array of Actor Object Reference"))
  (bind (_value _returnvalue) (`BlueprintMapLibrary.Map_Find` (`self.LifeTimeMap`) (`self.NumPoints`)))
  (bind (_value_2 _returnvalue_2) (`BlueprintMapLibrary.Map_Find` (`self.SpeedMap`) (`self.NumPoints`)))
  (`SplineComponent.ClearSplinePoints` (`self.Spline`) true)
  (for _array_element ActorArray
    (`SplineComponent.AddSplinePoint` (`self.Spline`) (+ (`self.K2_GetActorLocation` _array_element) (0.0 0.0 100.0)) "World" true)
    (`/Engine/EditorBlueprintResources/StandardMacros.IncrementInt` (`self.NumPoints`)))
  (`|ExecutionSequence`
    (:`then_0`
      (if _returnvalue
        (`NiagaraComponent.SetVariableFloat` (`self.NS_ShieldThrow`) "Lifetime" _value)))
    (:`then_1`
      (if _returnvalue_2
        (`NiagaraComponent.SetVariableFloat` (`self.NS_ShieldThrow`) "ShieldandTrailSpeed" _value_2)))
    (:`then_2`
      (`ActorComponent.Activate` (`self.NS_ShieldThrow`) false))))

(fn `UserConstructionScript`)